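; Configurable light fixture for the jail level, built as either a hanging lamp or a door light with an optional flicker.
; The construction script picks the mesh from IndexLigths and hides the light components the variant does not use.
; For the hanging lamp, ONOFF sets the lit or unlit material and spotlight visibility.
; When Anim is set, Tick fires an event that toggles the spotlight after a randomized sub-second Delay, producing irregular flicker.
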(event Custom|Anim_event
  (Utilities|FlowControl|Delay (Math|Random|RandomFloatinRange (Math|Random|RandomFloatinRange 0.1 0.4) (Math|Random|RandomFloatinRange 0.5 0.6)))
  (Rendering|ToggleVisibility (Variables|Default|GetSpotLight) false))

(event EventBeginPlay)

(event Collision|EventActorBeginOverlap
  (params (OtherActor :type Actor%20Object%20Reference)))

(event EventTick
  (params (DeltaSeconds :type Float%20%28single-precision%29))
  (if (Variables|Default|GetAnim)
    (CallFunction|AnimEvent)))

(fn ConstructionScript
  (bind _staticmesh (Variables|Default|GetStaticMesh))
  (bind _staticmesh_2 (Variables|Default|GetStaticMesh))
  (bind _spotlight (Variables|Default|GetSpotLight))
  (if (== (Variables|Default|GetIndex_ligths) 0)
    (Components|StaticMesh|SetStaticMesh _staticmesh "/Game/JAIL/Mesh/light_suspendu_static_mesh_static_mesh.light_suspendu_static_mesh_static_mesh")
    (if (Variables|Default|GetON/OFF)
      (Rendering|Material|SetMaterial _staticmesh_2 0 "/Game/jail/materials/Light_mat.Light_mat")
      (Rendering|SetVisibility _spotlight true false)
      (else
        (Rendering|Material|SetMaterial _staticmesh_2 0 "/Game/jail/materials/Light_off_mat.Light_off_mat")
        (Rendering|SetVisibility _spotlight false true)))
    (Rendering|SetVisibility (Variables|Default|GetPointLight) false true)
    (else
      (Components|StaticMesh|SetStaticMesh _staticmesh "/Game/JAIL/Mesh/light_door_static_mesh.light_door_static_mesh")
      (Rendering|SetVisibility (Variables|Default|GetSpotLight) false true))))