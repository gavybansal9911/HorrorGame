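; Straits_BP is a construction-time builder for a vertically repeating jail structure with light meshes and an optional grid.
; The Construction Script loops up to IndexStraits inclusive, adding local-space instances of the straits mesh and four light instance components at a fixed Z spacing.
; The Grid flag adds a matching grid instance at each level.
; The event graph's events are empty, so the Blueprint has no runtime logic.
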(event EventBeginPlay)

(event Collision|EventActorBeginOverlap
  (params (OtherActor :type Actor%20Object%20Reference)))

(event EventTick
  (params (DeltaSeconds :type Float%20%28single-precision%29)))

(fn ConstructionScript
  (for _index (range 0 (Variables|Default|GetIndex_straits))
    (Components|InstancedStaticMesh|AddInstance (Variables|Default|GetStraits_instance) (Math|Transform|MakeTransform (Math|Vector|MakeVector 0.0 0.0 (* _index 499.0))) false)
    (Components|InstancedStaticMesh|AddInstance (Variables|Default|GetLight) (Math|Transform|MakeTransform (Math|Vector|MakeVector 0.0 0.0 (* _index 499.0))) false)
    (Components|InstancedStaticMesh|AddInstance (Variables|Default|GetLight1) (Math|Transform|MakeTransform (Math|Vector|MakeVector 0.0 0.0 (* _index 499.0))) false)
    (Components|InstancedStaticMesh|AddInstance (Variables|Default|GetLight2) (Math|Transform|MakeTransform (Math|Vector|MakeVector 0.0 0.0 (* _index 499.0))) false)
    (Components|InstancedStaticMesh|AddInstance (Variables|Default|GetLight3) (Math|Transform|MakeTransform (Math|Vector|MakeVector 0.0 0.0 (* _index 499.0))) false)
    (if (Variables|Default|GetGrid?)
      (Components|InstancedStaticMesh|AddInstance (Variables|Default|GetStraits_grid_instance) (Math|Transform|MakeTransform (Math|Vector|MakeVector 0.0 0.0 (* _index 499.0))) false))))