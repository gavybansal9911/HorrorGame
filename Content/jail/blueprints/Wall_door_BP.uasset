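; Configurable jail wall-with-door actor whose look is set per instance in the editor.
; The construction script applies a wall material picked from an array by ID, then toggles visibility of the light, door, door chain variant and left or right wall chain from flags and indices.
; It has no runtime logic; the event graph holds only disabled placeholder events.
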(event EventBeginPlay)

(event Collision|EventActorBeginOverlap
  (params (OtherActor :type Actor%20Object%20Reference)))

(event EventTick
  (params (DeltaSeconds :type Float%20%28single-precision%29)))

(fn ConstructionScript
  (bind _chain_id (Variables|Default|GetChain_id))
  (bind _chaine_door (Variables|Default|Getchaine_door))
  (bind _chain_big (Variables|Default|Getchain_big))
  (bind _chain_wall_right (Variables|Default|Getchain_wall_right))
  (bind _chain_wall_left (Variables|Default|Getchain_wall_left))
  (bind _light (Variables|Default|Getlight))
  (bind _door (Variables|Default|Getdoor))
  (Utilities|FlowControl|Sequence
    (:then_0
      (Rendering|Material|SetMaterial (Variables|Default|Getwall) 0 (Utilities|Array|Get(acopy) (Variables|Default|GetMaterials) (Variables|Default|Getwall_id))))
    (:then_1
      (if (Variables|Default|GetLight%20?)
        (Rendering|SetVisibility _light true false)
        (else
          (Rendering|SetVisibility _light false true))))
    (:then_2
      (if (Variables|Default|GetDoor%20?)
        (Rendering|SetVisibility _door true false)
        (else
          (Rendering|SetVisibility _door false true))))
    (:then_3
      (if (Variables|Default|GetChain%20door%20?%20)
        (Utilities|FlowControl|Sequence
          (:then_0
            (if (== _chain_id 0)
              (Rendering|SetVisibility _chaine_door true false)
              (else
                (Rendering|SetVisibility _chaine_door false true))))
          (:then_1
            (if (== _chain_id 1)
              (Rendering|SetVisibility _chain_big true false)
              (else
                (Rendering|SetVisibility _chain_big false true)))))
        (else
          (Rendering|SetVisibility (Variables|Default|Getchaine_door) false true))))
    (:then_4
      (if (Variables|Default|GetChain%20wall%20?%20)
        (if (== (Variables|Default|GetChain%20position%20wall) 0)
          (Rendering|SetVisibility _chain_wall_right true false)
          (Rendering|SetVisibility _chain_wall_left false true)
          (else
            (Rendering|SetVisibility _chain_wall_right false true)
            (Rendering|SetVisibility _chain_wall_left true false)))
        (else
          (Rendering|SetVisibility _chain_wall_right false true)
          (Rendering|SetVisibility _chain_wall_left false true))))))