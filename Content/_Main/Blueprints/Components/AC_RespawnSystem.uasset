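; AC_RespawnSystem is an actor component that tracks the player's lives and respawns the first-person character.
; Lives start at the maximum on BeginPlay, and AddLife raises them within that cap.
; MinusLife decrements them, then either calls an empty EndGame stub at zero or moves the owner to a random respawn location, restoring walking and input.
; Tick prints the remaining lives as debug output.
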(event EventBeginPlay
  (CallFunction|Initialize))

(event EventTick
  (params (DeltaSeconds :type Float%20%28single-precision%29))
  (Development|PrintString (Utilities|String|ToString(Integer) (Variables|Default|GetLifes%20Remaining))))

(fn GetLifesRemaining
  (return (Variables|Default|GetLifes%20Remaining)))

(fn AddLife
  (params (Lifes%20To%20Add :type Integer))
  (Variables|Default|SetLifes%20Remaining (Math|Integer|Clamp(Integer) (+ (Variables|Default|GetLifes%20Remaining) Lifes%20To%20Add) 0 (Variables|Default|GetMax%20Lifes))))

(fn Initialize
  (Variables|Default|SetLifes%20Remaining (Variables|Default|GetMax%20Lifes)))

(fn MinusLife
  (Math|Integer|DecrementInt (Variables|Default|GetLifes%20Remaining)
    (:%20%20
      (CallFunction|CheckifGameEnd))))

(fn CheckifGameEnd
  (if (== (Variables|Default|GetLifes%20Remaining) 0)
    (Development|PrintString "GAME OVER!")
    (CallFunction|EndGame)
    (else
      (CallFunction|RespawnPlayer))))

(fn RespawnPlayer
  (bind _returnvalue (Game|GetPlayerController 0))
  (bind _asbp_first_person_character (Utilities|Casting|CastToBP_FirstPersonCharacter (Components|GetOwner)))
  (Transformation|SetActorLocation _asbp_first_person_character (.OutItem (Utilities|Array|Random (Variables|Default|GetRespawn%20Location))) false false)
  (Pawn|Components|CharacterMovement|SetMovementMode (Variables|/Script/Engine.Character|GetCharacterMovement _asbp_first_person_character) "MOVE_Walking" 0)
  (Input|EnableInput _asbp_first_person_character _returnvalue)
  (Input|SetIgnoreLookInput _returnvalue false))

(fn EndGame)