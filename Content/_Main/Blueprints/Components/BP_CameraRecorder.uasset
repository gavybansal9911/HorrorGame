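; Actor component on the first-person character that records in-game videos from its scene capture camera.
; While recording, each tick snapshots the render target into a static texture via an editor-only function and stores it in the current video's frame array.
; Starting a recording adds a new video entry.
; Stopping spawns a video cassette actor in front of the player, carrying that video's data.
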(event EventTick
  (params (DeltaSeconds :type Float%20%28single-precision%29))
  (bind _numberofvideos (Variables|Videos|GetNumberOfVideos))
  (bind _videos (Variables|Videos|GetVideos))
  (bind _videos_2 (Variables|Videos|GetVideos))
  (bind _numberofvideos_2 (Variables|Videos|GetNumberOfVideos))
  (bind _numberofvideos_3 (Variables|Videos|GetNumberOfVideos))
  (bind _videos_3 (Variables|Videos|GetVideos))
  (bind _numberofvideos_4 (Variables|Videos|GetNumberOfVideos))
  (bind _videos_4 (Variables|Videos|GetVideos))
  (bind _returnvalue (- _numberofvideos_3 1))
  (bind _returnvalue_2 (- _numberofvideos 1))
  (bind _returnvalue_3 (- _numberofvideos_2 1))
  (bind _returnvalue_4 (- _numberofvideos_4 1))
  (bind _output (Utilities|Array|Get(acopy) _videos_4 _returnvalue_2))
  (bind _output_2 (Utilities|Array|Get(acopy) _videos _returnvalue_3))
  (bind _output_3 (Utilities|Array|Get(acopy) _videos_3 _returnvalue_4))
  (bind _output_4 (Utilities|Array|Get(acopy) _videos_2 _returnvalue))
  (bind (_frametextures _lastindex) (Utilities|Struct|BreakFVideo _output_2))
  (bind (_frametextures_2 _lastindex_2) (Utilities|Struct|BreakFVideo _output_3))
  (bind (_frametextures_3 _lastindex_3) (Utilities|Struct|BreakFVideo _output))
  (bind (_frametextures_4 _lastindex_4) (Utilities|Struct|BreakFVideo _output_4))
  (if (Variables|Recording|GetbIsRecording)
    (bind _returnvalue_5 (Class|KismetRenderingLibrary|RenderTargetCreateStaticTexture2DEditorOnly (Variables|/Script/Engine.SceneCaptureComponent2D|GetTextureTarget (Variables|Ref|GetScene%20Capture%20Camera%20Ref)) (Utilities|String|MakeLiteralString (Utilities|String|ToString(Integer) (.LastIndex (Utilities|Struct|BreakFVideo (Utilities|Array|Get(acopy) (Variables|Videos|GetVideos) (- (Variables|Videos|GetNumberOfVideos) 1)))))) "TC_EditorIcon" "TMGS_FromTextureGroup"))
    (Utilities|Array|SetArrayElem _frametextures_4 _lastindex_4 _returnvalue_5)
    (Utilities|IsValid (Utilities|Array|Get(acopy) (.FrameTextures (Utilities|Struct|BreakFVideo (Utilities|Array|Get(acopy) (Variables|Videos|GetVideos) (- (Variables|Videos|GetNumberOfVideos) 1)))) _lastindex_4)
      (:Is%20Valid
        (Utilities|Array|SetArrayElem (Variables|Videos|GetVideos) (- (Variables|Videos|GetNumberOfVideos) 1) (Utilities|Struct|MakeFVideo _frametextures (+ _lastindex 1)))
        (Development|PrintString (Utilities|String|ToString(Integer) _lastindex_2))
        (Utilities|IsValid (Utilities|Array|Get(acopy) _frametextures_2 _lastindex_2)
          (:Is%20Valid
            _)
          (:Is%20Not%20Valid
            (Development|PrintString "Hello" true true "(R=1.000000,G=0.000000,B=0.274741,A=1.000000)")))
        (Utilities|Array|SetArrayElem (Variables|Videos|GetVideos) (- (Variables|Videos|GetNumberOfVideos) 1) (Utilities|Struct|MakeFVideo _frametextures_3 (+ _lastindex_3 1)))))))

(event EventBeginPlay
  (bind _asbp_first_person_character (Utilities|Casting|CastToBP_FirstPersonCharacter (Components|GetOwner)))
  (bind _output_get (Variables|Ref|SetPlayer%20Ref _asbp_first_person_character))
  (Variables|Ref|SetScene%20Capture%20Camera%20Ref (Variables|/Game/FirstPerson/Blueprints/BP_FirstPersonCharacter.BP_FirstPersonCharacter_C|GetSceneCaptureComponent2D _output_get)))

(fn StartRecording
  (bind _result (Math|Integer|IncrementInt (Variables|Videos|GetNumberOfVideos))
    (:%20%20
      (Utilities|Array|Resize (Variables|Videos|GetVideos) _result)
      (Variables|Recording|SetbIsRecording true))))

(fn StopRecording
  (bind _returnvalue (Game|GetPlayerCharacter 0))
  (Variables|Recording|SetbIsRecording false)
  (Game|SpawnActorfromClass "/Game/_Main/Blueprints/Actor/Inventory/BP_VideoCassete.BP_VideoCassete_C" (Math|Transform|MakeTransform (+ (Transformation|GetActorLocation _returnvalue) (* (Transformation|GetActorForwardVector _returnvalue) 25.0)) "0, 0, 0" "1.000000,1.000000,1.000000") "Undefined" "MultiplyWithRoot" 0 (Utilities|Array|Get(acopy) (Variables|Videos|GetVideos) (- (Variables|Videos|GetNumberOfVideos) 1)) 0))