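; AC_StateManager is a component that holds a character state and exposes functions to read, change and test it.
; The setter writes the new value only when it differs from the current one, and fires no notification on change.
; A query function loops over a supplied list of states and returns true on the first match with the current state, otherwise false.
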(fn GetCharacterState
  (return (Variables|Default|GetCharacter%20State)))

(fn SetCharacterState
  (params (In%20Character%20State :type ECharacterState%20Enum :default "NewEnumerator0"))
  (if (not (Utilities|Enum|Equal(Enum) In%20Character%20State (Variables|Default|GetCharacter%20State)))
    (Variables|Default|SetCharacter%20State In%20Character%20State)))

(fn IsCharacterStateEqualtoAny
  (params (States%20To%20Check :type Array%20of%20ECharacterState%20Enums :default "NewEnumerator0"))
  (for _array_element States%20To%20Check
    (if (Utilities|Enum|Equal(Enum) _array_element (Variables|Default|GetCharacter%20State))
      (return true)))
  (return false))