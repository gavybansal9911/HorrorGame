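; Actor component that manages flashlight battery life for BP_FirstPersonCharacter.
; Start and clear events control a looping timer that periodically lowers the clamped charge, with a debug message if started empty.
; Each tick of that timer prints the charge and updates the owner's HUD battery widget, then hides the flashlight and stops draining at zero.
; Getters and setters expose current and maximum battery life.
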(event Custom|Start%20Battery%20Drain
  (if (> (Variables|Default|GetCurrent%20Battery%20Life) 0.0)
    (Utilities|Time|SetTimerbyFunctionName 0 "Battery Drain Update" 2.5 true)
    (else
      (Development|PrintString "Need Battery!"))))

(event Custom|Clear%20Battery%20drain
  (Utilities|Time|ClearTimerbyFunctionName 0 "Battery Drain Update"))

(fn BatteryDrainUpdate
  (if (> (Variables|Default|GetCurrent%20Battery%20Life) 0.0)
    (Variables|Default|SetCurrent%20Battery%20Life (Math|Float|Clamp(Float) (- (Variables|Default|GetCurrent%20Battery%20Life) 4.0) 0.0 (Variables|Default|GetMax%20Battery%20Life)))
    (Development|PrintString (Utilities|String|ToString(Float) (Variables|Default|GetCurrent%20Battery%20Life)))
    (Default|UpdateBattery (Variables|/Game/_Main/UI/WBP_MainHud.WBP_MainHud_C|GetW_FlashlightBattery (Variables|/Game/FirstPerson/Blueprints/BP_FirstPersonCharacter.BP_FirstPersonCharacter_C|GetMain%20HUD (.AsBP%20First%20Person%20Character (Utilities|Casting|CastToBP_FirstPersonCharacter (Components|GetOwner))))) (Variables|Default|GetCurrent%20Battery%20Life) (Variables|Default|GetMax%20Battery%20Life))
    (if (not (> (Variables|Default|GetCurrent%20Battery%20Life) 0.0))
      (Rendering|SetVisibility (Variables|/Game/FirstPerson/Blueprints/BP_FirstPersonCharacter.BP_FirstPersonCharacter_C|GetFlashlight (.AsBP%20First%20Person%20Character (Utilities|Casting|CastToBP_FirstPersonCharacter (Components|GetOwner)))) false false)
      (CallFunction|ClearBatteryDrain))))

(fn GetCurrentBatteryLife
  (return (Variables|Default|GetCurrent%20Battery%20Life)))

(fn GetMaxBatteryLife
  (return (Variables|Default|GetMax%20Battery%20Life)))

(fn SetMaxBatteryLife
  (params (New%20Max%20Battery%20Life :type Float%20%28double-precision%29))
  (Variables|Default|SetMax%20Battery%20Life New%20Max%20Battery%20Life))

(fn SetCurrentBatteryLife
  (params (Current%20Battery%20Life :type Float%20%28double-precision%29))
  (Variables|Default|SetCurrent%20Battery%20Life (Math|Float|Clamp(Float) Current%20Battery%20Life 0.0 (Variables|Default|GetMax%20Battery%20Life))))