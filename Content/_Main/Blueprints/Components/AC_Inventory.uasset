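; Inventory component for BP_FirstPersonCharacter that stores items in a fixed-size slot array and handles adding, using, inspecting and dropping.
; Adding tops up matching stacks before filling empty slots, recursing on overflow and firing an inventory-updated event.
; Item actions message actors of the item's class; inspect also opens W_Inspection.
; Drop removes one unit but spawns an actor carrying the slot's prior quantity at a camera trace point.
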(event EventBeginPlay
  (CallFunction|Initialize))

(fn Initialize
  (Utilities|Array|Resize (Variables|Data|GetContent) (Variables|InventoryProperties|GetInventory%20Size))
  (bind _asbp_first_person_character (Utilities|Casting|CastToBP_FirstPersonCharacter (Components|GetOwner)))
  (Variables|Default|SetPlayer%20Ref _asbp_first_person_character)
  (bind _returnvalue (UserInterface|CreateWidget "/Game/_Main/UI/W_Inspection.W_Inspection_C" 0 self))
  (Variables|Default|SetW%20Inspection%20Ref _returnvalue)
  (bind _outactors (Actor|GetAllActorsOfClass "/Game/_Main/Blueprints/Actor/Inspection/BP_Inspection.BP_Inspection_C"))
  (Variables|Default|SetBP%20Inspection%20Ref (Utilities|Array|Get(acopy) _outactors)))

(fn PrintContentData
  (for _array_element (Variables|Data|GetContent)
    (Development|PrintString (Utilities|String|ToString(Text) (Utilities|Text|FormatText "{ItemName}: {Quantity}" (.itemname (.ItemData (Utilities|Struct|BreakFInventoryActorData _array_element))) (.Quantity (Utilities|Struct|BreakFInventoryActorData _array_element)))))))

(fn AddItemtoInventory
  (params (Inventory%20Actor%20Data :type F%20Inventory%20Actor%20Data%20Structure))
  (bind (_bavailable _index) (CallFunction|EmptySlotAvailable))
  (bind (_bavailable_2 _index_2) (CallFunction|ExistingSlotAvailable (.itemid Inventory%20Actor%20Data)))
  (if _bavailable_2
    (bind (_badded_ _quantity_remaining) (CallFunction|AddItemtoExistingSlot Inventory%20Actor%20Data _index_2))
    (if _badded_
      (if (== _quantity_remaining 0)
        (Default|CallOnInventoryUpdated)
        (return true 0)
        (else
          (bind _quantity_remaining_2 (CallFunction|AddItemtoInventory (Utilities|Struct|MakeFInventoryActorData (.itemid Inventory%20Actor%20Data) _quantity_remaining (.itemdata Inventory%20Actor%20Data))))
          (Default|CallOnInventoryUpdated)
          (return true _quantity_remaining_2))))
    (elif _bavailable
      (bind (_created _quantity_remaining_3) (CallFunction|CreateNewStack _index Inventory%20Actor%20Data))
      (Default|CallOnInventoryUpdated)
      (return _created _quantity_remaining_3)
      (else
        (Default|CallOnInventoryUpdated)
        (return false (Utilities|Struct|BreakFInventoryActorData Inventory%20Actor%20Data))))))

(fn GetDataatIndex
  (params (index :type Integer))
  (if (> index (- (Variables|InventoryProperties|GetInventory%20Size) 1))
    (return false "")
    (else
      (return true (Utilities|Array|Get(acopy) (Variables|Data|GetContent) index)))))

(fn ExistingSlotAvailable
  (params (Item%20ID :type Name))
  (bind (_array_element _array_index) (Utilities|Array|ForEachLoopwithBreak (Variables|Data|GetContent) :!label _label)
    (:LoopBody
      (if (and (== Item%20ID (.ItemID (Utilities|Struct|BreakFInventoryActorData _array_element))) (> (.maxstacksize (.ItemData (Utilities|Struct|BreakFInventoryActorData _array_element))) (.Quantity (Utilities|Struct|BreakFInventoryActorData _array_element))))
        (LocalVariables|SetLocal_Success true)
        (LocalVariables|SetLocal_Index _array_index)
        (goto _label Break)))
    (:Completed
      (return (LocalVariables|GetLocal_Success) (LocalVariables|GetLocal_Index)))))

(fn EmptySlotAvailable
  (for (_array_element _array_index) (Variables|Data|GetContent)
    (if (== (.Quantity (Utilities|Struct|BreakFInventoryActorData _array_element)) 0)
      (return true _array_index)))
  (return false -1))

(fn CreateNewStack
  (params (Index :type Integer) (InventoryActorData :type F%20Inventory%20Actor%20Data%20Structure))
  (if (not (> (.quantity InventoryActorData) (.maxstacksize (.itemdata InventoryActorData))))
    (Utilities|Array|SetArrayElem (Variables|Data|GetContent) Index InventoryActorData)
    (return true 0)
    (else
      (Utilities|Array|SetArrayElem (Variables|Data|GetContent) Index (Utilities|Struct|MakeFInventoryActorData (.itemid InventoryActorData) (.MaxStackSize (Utilities|Struct|BreakFItemData (.itemdata InventoryActorData))) (.itemdata InventoryActorData)))
      (bind _quantity_remaining (CallFunction|AddItemtoInventory (Utilities|Struct|MakeFInventoryActorData (.itemid InventoryActorData) (- (.quantity InventoryActorData) (.MaxStackSize (Utilities|Struct|BreakFItemData (.itemdata InventoryActorData)))) (.itemdata InventoryActorData))))
      (return true _quantity_remaining))))

(fn AddItemtoExistingSlot
  (params (Inventory%20Actor%20Data :type F%20Inventory%20Actor%20Data%20Structure) (Index :type Integer))
  (bind (_quantity _itemdata) (Utilities|Struct|BreakFInventoryActorData Inventory%20Actor%20Data))
  (bind _content (Variables|Data|GetContent))
  (bind _output (Utilities|Array|Get(acopy) _content Index))
  (LocalVariables|SetLocal_QuantityRemaining _quantity)
  (if (> (+ _quantity (.quantity (Utilities|Array|Get(acopy) (Variables|Data|GetContent) Index))) (.MaxStackSize (Utilities|Struct|BreakFItemData _itemdata)))
    (LocalVariables|SetLocal_QuantityAtIndex (.quantity (Utilities|Array|Get(acopy) (Variables|Data|GetContent) Index)))
    (Utilities|Array|SetArrayElem (Variables|Data|GetContent) Index (Utilities|Struct|MakeFInventoryActorData (.itemid Inventory%20Actor%20Data) (.MaxStackSize (Utilities|Struct|BreakFItemData (.itemdata Inventory%20Actor%20Data))) (.itemdata Inventory%20Actor%20Data)))
    (LocalVariables|SetLocal_QuantityRemaining (- (.quantity Inventory%20Actor%20Data) (- (.MaxStackSize (Utilities|Struct|BreakFItemData (.itemdata Inventory%20Actor%20Data))) (LocalVariables|GetLocal_QuantityAtIndex))))
    (LocalVariables|SetLocal_QuantityAtIndex (.MaxStackSize (Utilities|Struct|BreakFItemData (.itemdata Inventory%20Actor%20Data))))
    (bind _quantity_remaining (CallFunction|AddItemtoInventory (Utilities|Struct|MakeFInventoryActorData (.itemid Inventory%20Actor%20Data) (LocalVariables|GetLocal_QuantityRemaining) (.itemdata Inventory%20Actor%20Data))))
    (return true _quantity_remaining)
    (else
      (Utilities|Array|SetArrayElem (Variables|Data|GetContent) Index (Utilities|Struct|MakeFInventoryActorData (.itemid _output) (+ (.quantity _output) (.quantity Inventory%20Actor%20Data)) (.itemdata Inventory%20Actor%20Data)))
      (return true 0))))

(fn UpdateInventory
  (for (_ _array_index) (Variables|Data|GetContent)
    (CallFunction|UpdateSlot _array_index)))

(fn UpdateSlot
  (params (Index :type Integer))
  (if (.bSuccess (Utilities|Casting|CastToBP_FirstPersonCharacter (Components|GetOwner)))
    _))

(fn UseItematIndex
  (params (Index :type Integer))
  (bind _content (Variables|Data|GetContent))
  (bind _output (Utilities|Array|Get(acopy) _content Index))
  (bind _itemclass (Utilities|Struct|BreakFItemData (.itemdata _output)))
  (if (> (.quantity _output) 0)
    (bind _returnvalue (Actor|GetActorOfClass _itemclass))
    (Utilities|IsValid _returnvalue
      (:Is%20Valid
        (Class|IInventoryItemInterface|UseItem(Message) _returnvalue)
        (CallFunction|RemoveItematIndex Index))
      (:Is%20Not%20Valid
        (bind _returnvalue_2 (Game|SpawnActorfromClass _itemclass (Math|Transform|MakeTransform "0, 0, 0" "0, 0, 0" "1.000000,1.000000,1.000000") "Undefined" "MultiplyWithRoot" 0 0))
        (Class|IInventoryItemInterface|UseItem(Message) _returnvalue_2)
        (CallFunction|RemoveItematIndex Index)))))

(fn InspectItematIndex
  (params (Index :type Integer))
  (bind _returnvalue (Actor|GetActorOfClass (.ItemClass (Utilities|Struct|BreakFItemData (.itemdata (Utilities|Array|Get(acopy) (Variables|Data|GetContent) Index))))))
  (Class|IInventoryItemInterface|InspectItem(Message) _returnvalue)
  (CallFunction|CreateInspectionWidget Index))

(fn DropItematIndex
  (params (index :type Integer))
  (bind _return_value (CallFunction|GetDataatIndex index))
  (bind _player_ref (Variables|Default|GetPlayer%20Ref))
  (bind _itemclass (Utilities|Struct|BreakFItemData (.itemdata _return_value)))
  (bind _firstpersoncamera (Variables|/Game/FirstPerson/Blueprints/BP_FirstPersonCharacter.BP_FirstPersonCharacter_C|GetFirstPersonCamera _player_ref))
  (bind _returnvalue (Transformation|GetWorldLocation _firstpersoncamera))
  (LocalVariables|SetLocal_Quantity (.quantity _return_value))
  (if (> (.quantity _return_value) 0)
    (LocalVariables|SetLocal_ItemClass _itemclass)
    (bind _returnvalue_2 (Actor|GetActorOfClass _itemclass))
    (Class|IInventoryItemInterface|DropItem(Message) _returnvalue_2)
    (CallFunction|RemoveItematIndex index)
    (bind (_outhit _returnvalue_3) (Collision|LineTraceByChannel _returnvalue (+ _returnvalue (* (Math|Vector|GetForwardVector _firstpersoncamera) 1e+02)) "TraceTypeQuery1" false 0 "None"))
    (bind _returnvalue_4 (Game|SpawnActorfromClass (LocalVariables|GetLocal_ItemClass) (Math|Transform|MakeTransform (select _returnvalue_3 (.Location (Collision|BreakHitResult _outhit)) (.TraceEnd (Collision|BreakHitResult _outhit))) "0, 0, 0" "1.000000,1.000000,1.000000") "Undefined" "MultiplyWithRoot" 0 0))
    (Variables|/Game/_Main/Blueprints/Actor/Inventory/BP_InventoryItemBase.BP_InventoryItemBase_C|SetQuantity _returnvalue_4 (LocalVariables|GetLocal_Quantity))))

(fn DropAllItematIndex
  (params (Index :type Integer)))

(fn RemoveItematIndex
  (params (Index :type Integer))
  (bind _return_value (CallFunction|GetDataatIndex Index))
  (if (> (.quantity (.Return%20value (CallFunction|GetDataatIndex Index))) 1)
    (Utilities|Array|SetArrayElem (Variables|Data|GetContent) Index (Utilities|Struct|MakeFInventoryActorData (.itemid _return_value) (- (.quantity _return_value) 1) (.itemdata _return_value)))
    (Default|CallOnInventoryUpdated)
    (else
      (Utilities|Array|SetArrayElem :TargetArray (Variables|Data|GetContent) :Index Index)
      (Default|CallOnInventoryUpdated))))

(fn CreateInspectionWidget
  (params (Index :type Integer))
  (Default|UpdateWidget (Variables|Default|GetW%20Inspection%20Ref) Index)
  (Widget|SetVisibility (Variables|/Game/FirstPerson/Blueprints/BP_FirstPersonCharacter.BP_FirstPersonCharacter_C|GetInventory%20Menu%20Ref (Variables|Default|GetPlayer%20Ref)) "Hidden")
  (UserInterface|Viewport|AddtoViewport (Variables|Default|GetW%20Inspection%20Ref) 2))