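; Actor component that tracks game objectives and shows the active one in an on-screen objective widget.
; On BeginPlay it creates the objective layer widget and displays the first remaining objective, without setting it as current.
; Assigning an objective sets it as current and updates the widget text.
; Completing one moves it from the remaining to the completed list and clears it, with both actions firing notification calls.
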(event EventBeginPlay
  (Initialize|Initialize))

(fn CompleteObjective
  (Utilities|Array|RemoveItem (Variables|ObjectiveData|GetObjectives%20Remaining) (Variables|ObjectiveData|GetCurrent%20Objective))
  (Utilities|Array|AddUnique (Variables|CompletedObjectiveData|GetObjectives%20Completed) (Variables|ObjectiveData|GetCurrent%20Objective))
  (Variables|ObjectiveData|SetCurrent%20Objective "")
  (Default|CallOnObjectiveCompleted))

(fn AssignNewObjective
  (params (New%20Objective :type F%20Objective%20Data%20Structure))
  (bind _output_get (Variables|ObjectiveData|SetCurrent%20Objective New%20Objective))
  (UI|UpdateUIText (Utilities|Text|ToText(Name) (.ObjectiveName (Utilities|Struct|BreakFObjectiveData _output_get))) (.Objective (Utilities|Struct|BreakFObjectiveData _output_get)))
  (Default|CallOnObjectiveAssigned))

(fn Initialize
  (bind _objectives_remaining (Variables|ObjectiveData|GetObjectives%20Remaining))
  (bind _output (Utilities|Array|Get(acopy) _objectives_remaining))
  (bind (_objectivename _objectiveindex _objective) (Utilities|Struct|BreakFObjectiveData _output))
  (bind _returnvalue (UserInterface|CreateWidget "/Game/_Main/UI/ObjectiveSystem/W_ObjectiveLayer.W_ObjectiveLayer_C" 0 "None"))
  (bind _output_get (Variables|UI|SetObject%20Layer%20UI _returnvalue))
  (UserInterface|Viewport|AddtoViewport _output_get 5)
  (UI|UpdateUIText (Utilities|Text|ToText(Name) _objectivename) _objective))

(fn UpdateUIText
  (params (Objective%20Name :type Text) (Objective%20Text :type Text))
  (Variables|/Game/_Main/UI/ObjectiveSystem/W_ObjectiveLayer.W_ObjectiveLayer_C|SetObjective%20Name (Variables|UI|GetObject%20Layer%20UI) Objective%20Name)
  (Variables|/Game/_Main/UI/ObjectiveSystem/W_ObjectiveLayer.W_ObjectiveLayer_C|SetObjective%20Text (Variables|UI|GetObject%20Layer%20UI) Objective%20Text))

(fn GetCurrentObjective
  (return (Variables|ObjectiveData|GetCurrent%20Objective)))