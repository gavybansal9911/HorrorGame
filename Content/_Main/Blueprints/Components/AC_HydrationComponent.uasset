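; AC_HydrationComponent is an actor component that stores a current and maximum hydration value for its owner.
; Getter and setter functions expose both values, and setting current hydration clamps it between zero and the maximum.
; Setting the maximum does not re-clamp the current value, and Tick holds no logic, so hydration changes only through these setters.
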(event EventTick
  (params (DeltaSeconds :type Float%20%28single-precision%29)))

(fn GetCurrentHydration
  (return (Variables|Default|GetCurrent%20Hydration)))

(fn GetMaxHydration
  (return (Variables|Default|GetMax%20Hydration)))

(fn SetCurrentHydration
  (params (New%20Current%20Hydration :type Float%20%28double-precision%29))
  (Variables|Default|SetCurrent%20Hydration (Math|Float|Clamp(Float) New%20Current%20Hydration 0.0 (Variables|Default|GetMax%20Hydration))))

(fn SetMaxHydration
  (params (New%20Max%20Hydration :type Float%20%28double-precision%29))
  (Variables|Default|SetMax%20Hydration New%20Max%20Hydration))