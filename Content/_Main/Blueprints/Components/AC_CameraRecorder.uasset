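; Actor component that records video from the first-person character's scene capture camera as a sequence of textures.
; On BeginPlay it caches the owning BP_FirstPersonCharacter's SceneCaptureComponent2D.
; While recording, each Tick converts the render target into a static texture with an editor-only function and appends it to VideoData, advancing the frame index.
; StartRecording sets the flag; StopRecording is empty, so nothing here clears it.
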(event EventBeginPlay
  (bind _asbp_first_person_character (Utilities|Casting|CastToBP_FirstPersonCharacter (Components|GetOwner)))
  (Variables|Default|SetScene%20Capture%20Camera%20Ref (Variables|/Game/FirstPerson/Blueprints/BP_FirstPersonCharacter.BP_FirstPersonCharacter_C|GetSceneCaptureComponent2D _asbp_first_person_character)))

(event EventTick
  (params (DeltaSeconds :type Float%20%28single-precision%29))
  (if (Variables|Default|GetbRecording)
    (Utilities|Array|Resize (.frametextures (Variables|Default|GetVideoData)) (+ (.lastindex (Variables|Default|GetVideoData)) 1))
    (bind _returnvalue (Class|KismetRenderingLibrary|RenderTargetCreateStaticTexture2DEditorOnly (Variables|/Script/Engine.SceneCaptureComponent2D|GetTextureTarget (Variables|Default|GetScene%20Capture%20Camera%20Ref)) (Utilities|String|ToString(Integer) (.LastIndex (Utilities|Struct|BreakFVideo (Variables|Default|GetVideoData)))) "TC_EditorIcon" "TMGS_FromTextureGroup"))
    (Utilities|Array|SetArrayElem (.frametextures (Variables|Default|GetVideoData)) (.lastindex (Variables|Default|GetVideoData)) _returnvalue)
    (Variables|Default|SetVideoData (Utilities|Struct|MakeFVideo (.frametextures (Variables|Default|GetVideoData)) (+ (.lastindex (Variables|Default|GetVideoData)) 1)))))

(fn StartRecording
  (Variables|Default|SetbRecording true))

(fn StopRecording)