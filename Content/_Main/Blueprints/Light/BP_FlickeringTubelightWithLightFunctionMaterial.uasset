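; Tubelight actor that flickers a rect light, with an optional light function material applied in the construction script.
; BeginPlay starts flickering if the Flicker flag is set, and the Flicker event sets that flag and starts it.
; A looping retriggerable delay of random length drives a FlipFlop that alternates between minimum flicker and normal intensity.
; UnFlicker only clears the flag, which the running loop never rechecks.
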(event Custom|Flicker
  (Variables|Default|SetbFlicker true)
  (if (Variables|Default|GetbFlicker)
    (Utilities|FlowControl|RetriggerableDelay (Math|Random|RandomFloatinRange (Variables|Default|GetMin%20Time) (Variables|Default|GetMax%20Time)) :!label _label)
    (Utilities|FlowControl|FlipFlop
      (:A
        (Rendering|Components|Light|SetIntensity (Variables|Default|GetRectLight) (Variables|Default|GetMin%20Flicker%20Intensity))
        (goto _label))
      (:B
        (Rendering|Components|Light|SetIntensity (Variables|Default|GetRectLight) (Variables|Default|GetIntensity))
        (goto _label)))))

(event Custom|UnFlicker
  (Variables|Default|SetbFlicker false))

(event EventBeginPlay
  (if (Variables|Default|GetbFlicker)
    (Utilities|FlowControl|RetriggerableDelay (Math|Random|RandomFloatinRange (Variables|Default|GetMin%20Time) (Variables|Default|GetMax%20Time)) :!label _label)
    (Utilities|FlowControl|FlipFlop
      (:A
        (Rendering|Components|Light|SetIntensity (Variables|Default|GetRectLight) (Variables|Default|GetMin%20Flicker%20Intensity))
        (goto _label))
      (:B
        (Rendering|Components|Light|SetIntensity (Variables|Default|GetRectLight) (Variables|Default|GetIntensity))
        (goto _label)))))

(fn ConstructionScript
  (Rendering|Components|Light|SetIntensity (Variables|Default|GetRectLight) (Variables|Default|GetIntensity))
  (if (Variables|Default|GetbUseLightFunctionMaterial)
    (Rendering|Components|Light|SetLightFunctionMaterial (Variables|Default|GetRectLight) (Variables|Default|GetLight%20Function%20Material))))