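; Base actor for world items that the player can pick up into an inventory, carrying an inventory data struct of ID, quantity and item data.
; BeginPlay rebuilds that struct with the actor's Quantity variable.
; Interacting passes it to the player's inventory component, then keeps any leftover quantity or destroys the actor once fully added.
; Inspect, drop and use only print placeholder messages, and Look At returns empty text.
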(event EventBeginPlay
  (Variables|Inventory|SetActor%20Data (Utilities|Struct|MakeFInventoryActorData (.ItemID (Utilities|Struct|BreakFInventoryActorData (Variables|Inventory|GetActor%20Data))) (Variables|Inventory|GetQuantity) (.ItemData (Utilities|Struct|BreakFInventoryActorData (Variables|Inventory|GetActor%20Data))))))

(event EventInspectItem
  (Development|PrintString "Inspect Item Called from BP_InventoryItemBase"))

(event EventDropItem
  (Development|PrintString "Drop Item Called from BP_InventoryItemBase"))

(event EventInteractwith
  (params (Player%20Character :type BP%20First%20Person%20Character%20Object%20Reference) (Grabbed%20Item :type BP%20Grab%20Item%20Base%20Object%20Reference) (Hit%20Component :type Primitive%20Component%20Object%20Reference))
  (bind (_added _quantity_remaining) (Default|AddItemtoInventory (Variables|/Game/FirstPerson/Blueprints/BP_FirstPersonCharacter.BP_FirstPersonCharacter_C|GetAC_Inventory Player%20Character) (Variables|Inventory|GetActor%20Data)))
  (if _added
    (if (> _quantity_remaining 0)
      (Variables|Inventory|SetActor%20Data (Utilities|Struct|MakeFInventoryActorData (.itemid (Variables|Inventory|GetActor%20Data)) _quantity_remaining (.itemdata (Variables|Inventory|GetActor%20Data))))
      (else
        (Actor|DestroyActor)))))

(fn ConstructionScript)

(fn Lookat
  (return ""))

(fn UseItem
  (Development|PrintString "use Item Called from BP_InventoryItemBase")
  (return false))