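; BP_EmptyPhotoPaper is an inventory item for blank photo paper that the player loads into their camera.
; Its Use Item override sets HavePaperEnteredForPhoto on the player's ACCameraRecorder component and returns true, or returns false if paper is already loaded.
; The On, Off and InspectItem events are empty, and BeginPlay and construction only call the parent.
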(event EventBeginPlay
  (|CallParentFunction))

(event EventOff)

(event EventOn)

(event EventInspectItem)

(fn ConstructionScript
  (|CallParentFunction))

(fn UseItem
  (bind _player_character (CallFunction|GetMyPlayerCharacter))
  (bind _ac_camerarecorder (Variables|/Game/FirstPerson/Blueprints/BP_FirstPersonCharacter.BP_FirstPersonCharacter_C|GetAC_CameraRecorder _player_character))
  (if (Variables|/Game/_Main/Blueprints/Components/AC_CameraRecorder.AC_CameraRecorder_C|GetbHavePaperEnteredForPhoto _ac_camerarecorder)
    (return false)
    (else
      (Variables|/Game/_Main/Blueprints/Components/AC_CameraRecorder.AC_CameraRecorder_C|SetbHavePaperEnteredForPhoto _ac_camerarecorder true)
      (return true))))