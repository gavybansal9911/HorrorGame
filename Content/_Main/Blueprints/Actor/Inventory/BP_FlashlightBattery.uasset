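; BP_FlashlightBattery is an inventory item that recharges the player's flashlight when used.
; UseItem casts the player to BP_FirstPersonCharacter, adds BatteryIncrementValue to the flashlight component's battery life and returns whether the cast succeeded.
; It then updates the HUD battery widget, re-reading battery life after the set and adding the increment again for the displayed value.
; LookAt returns an empty string.
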(fn ConstructionScript
  (|CallParentFunction))

(fn Lookat
  (return ""))

(fn UseItem
  (bind _asbp_first_person_character (Utilities|Casting|CastToBP_FirstPersonCharacter (Game|GetPlayerCharacter 0))
    (:then
      (Default|SetCurrentBatteryLife (Variables|/Game/FirstPerson/Blueprints/BP_FirstPersonCharacter.BP_FirstPersonCharacter_C|GetAC_FlashlightComponent _asbp_first_person_character) (+ (Default|GetCurrentBatteryLife (Variables|/Game/FirstPerson/Blueprints/BP_FirstPersonCharacter.BP_FirstPersonCharacter_C|GetAC_FlashlightComponent _asbp_first_person_character)) (Variables|Default|GetBattery%20Increment%20Value)))
      (Default|UpdateBattery (Variables|/Game/_Main/UI/WBP_MainHud.WBP_MainHud_C|GetW_FlashlightBattery (Variables|/Game/FirstPerson/Blueprints/BP_FirstPersonCharacter.BP_FirstPersonCharacter_C|GetMain%20HUD _asbp_first_person_character)) (+ (Default|GetCurrentBatteryLife (Variables|/Game/FirstPerson/Blueprints/BP_FirstPersonCharacter.BP_FirstPersonCharacter_C|GetAC_FlashlightComponent _asbp_first_person_character)) (Variables|Default|GetBattery%20Increment%20Value)) (Default|GetMaxBatteryLife (Variables|/Game/FirstPerson/Blueprints/BP_FirstPersonCharacter.BP_FirstPersonCharacter_C|GetAC_FlashlightComponent _asbp_first_person_character)))
      (return true))
    (:CastFailed
      (return false))))