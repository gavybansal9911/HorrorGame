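; BP_UnusableItem is an inventory item actor whose Use Item function changes the player's hydration, despite the "Unusable" in its name.
; Use Item casts player character 0 to BP_FirstPersonCharacter and adds HydrationIncrementValue to the current value on its ACHydrationComponent, clamped between zero and the maximum.
; The construction script only calls its parent's.
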(fn ConstructionScript
  (|CallParentFunction))

(fn UseItem
  (bind _asbp_first_person_character (Utilities|Casting|CastToBP_FirstPersonCharacter (Game|GetPlayerCharacter 0)))
  (Default|SetCurrentHydration (Variables|/Game/FirstPerson/Blueprints/BP_FirstPersonCharacter.BP_FirstPersonCharacter_C|GetAC_HydrationComponent _asbp_first_person_character) (Math|Float|Clamp(Float) (+ (Default|GetCurrentHydration (Variables|/Game/FirstPerson/Blueprints/BP_FirstPersonCharacter.BP_FirstPersonCharacter_C|GetAC_HydrationComponent _asbp_first_person_character)) (Variables|Default|GetHydration%20Increment%20Value)) 0.0 (Default|GetMaxHydration (Variables|/Game/FirstPerson/Blueprints/BP_FirstPersonCharacter.BP_FirstPersonCharacter_C|GetAC_HydrationComponent _asbp_first_person_character))))
  (return))