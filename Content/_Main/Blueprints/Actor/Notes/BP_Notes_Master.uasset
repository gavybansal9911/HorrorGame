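; Master Blueprint for an inspectable note that shows a prompt when the first-person character overlaps its sphere.
; Interacting moves the note in front of the camera and transfers input from the player to the note.
; Mouse wheel zooms via clamped camera FOV, and left-button drag rotates the paper in fixed steps.
; Backspace returns input and restores the paper's transform cached at construction, where its text is also set.
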(event OnComponentBeginOverlap(OverlapSphere)
  (params (OverlappedComponent :type Primitive%20Component%20Object%20Reference) (OtherActor :type Actor%20Object%20Reference) (OtherComp :type Primitive%20Component%20Object%20Reference) (OtherBodyIndex :type Integer) (bFromSweep :type Boolean) (SweepResult :type Hit%20Result%20Structure%20%28by%20ref%29))
  (Utilities|Casting|CastToBP_FirstPersonCharacter OtherActor)
  (Rendering|SetVisibility (Variables|Default|GetPrompt) true false))

(event OnComponentEndOverlap(OverlapSphere)
  (params (OverlappedComponent :type Primitive%20Component%20Object%20Reference) (OtherActor :type Actor%20Object%20Reference) (OtherComp :type Primitive%20Component%20Object%20Reference) (OtherBodyIndex :type Integer))
  (Utilities|Casting|CastToBP_FirstPersonCharacter OtherActor)
  (Rendering|SetVisibility (Variables|Default|GetPrompt) false false))

(event EventInteractwith
  (params (Player%20Character :type BP%20First%20Person%20Character%20Object%20Reference) (Grabbed%20Item :type BP%20Grab%20Item%20Base%20Object%20Reference) (Hit%20Component :type Primitive%20Component%20Object%20Reference))
  (bind _returnvalue (Game|GetPlayerController 0))
  (bind _firstpersoncamera (Variables|/Game/FirstPerson/Blueprints/BP_FirstPersonCharacter.BP_FirstPersonCharacter_C|GetFirstPersonCamera Player%20Character))
  (Variables|Default|SetFirst%20Person%20Camera _firstpersoncamera)
  (Transformation|SetWorldLocation (Variables|Default|GetBase%20Mesh) (+ (Transformation|GetWorldLocation _firstpersoncamera) (* (Math|Vector|GetForwardVector _firstpersoncamera) 1e+02)) false false)
  (Variables|Default|SetMaxFOV (Variables|/Script/Engine.CameraComponent|GetFieldOfView _firstpersoncamera))
  (Input|DisableInput Player%20Character _returnvalue)
  (Input|EnableInput self _returnvalue)
  (Rendering|SetVisibility (Variables|Default|GetPrompt) false false))

(event EventRelease)

(event EventGrab
  (params (Player%20Character :type BP%20First%20Person%20Character%20Object%20Reference) (Hit%20Location :type Vector :default "0, 0, 0")))

(event Input|MouseEvents|MouseX
  (params (AxisValue :type Float%20%28single-precision%29))
  (bind _paper_mesh (Variables|Default|GetPaper%20Mesh))
  (bind _relativerotation (Variables|/Script/Engine.SceneComponent|GetRelativeRotation _paper_mesh))
  (if (and (!= AxisValue 0.0) (Game|Player|IsInputKeyDown (Game|GetPlayerController 0) "LeftMouseButton"))
    (Transformation|SetRelativeRotation (Variables|Default|GetPaper%20Mesh) (Math|Rotator|MakeRotator (.roll _relativerotation) (.pitch _relativerotation) (select (> AxisValue 0.0) (- (.yaw _relativerotation) 2.0) (+ (.yaw _relativerotation) 2.0))) false false)))

(event Input|MouseEvents|MouseY
  (params (AxisValue :type Float%20%28single-precision%29))
  (bind _paper_mesh (Variables|Default|GetPaper%20Mesh))
  (bind _relativerotation (Variables|/Script/Engine.SceneComponent|GetRelativeRotation _paper_mesh))
  (if (and (!= AxisValue 0.0) (Game|Player|IsInputKeyDown (Game|GetPlayerController 0) "LeftMouseButton"))
    (Transformation|SetRelativeRotation (Variables|Default|GetPaper%20Mesh) (Math|Rotator|MakeRotator (.roll _relativerotation) (select (> AxisValue 0.0) (- (.pitch _relativerotation) 2.0) (+ (.pitch _relativerotation) 2.0)) (.yaw _relativerotation)) false false)))

(event Input|MouseEvents|MouseWheelUp
  (params (Key :type Key%20Structure :default "None"))
  (:Pressed
    (Variables|/Script/Engine.CameraComponent|SetFieldOfView (Variables|Default|GetFirst%20Person%20Camera) (Math|Float|Clamp(Float) (- (Variables|/Script/Engine.CameraComponent|GetFieldOfView (Variables|Default|GetFirst%20Person%20Camera)) 5.0) (Variables|Default|GetMinFOV) (Variables|Default|GetMaxFOV)))))

(event Input|MouseEvents|MouseWheelDown
  (params (Key :type Key%20Structure :default "None"))
  (:Pressed
    (Variables|/Script/Engine.CameraComponent|SetFieldOfView (Variables|Default|GetFirst%20Person%20Camera) (Math|Float|Clamp(Float) (+ (Variables|/Script/Engine.CameraComponent|GetFieldOfView (Variables|Default|GetFirst%20Person%20Camera)) 5.0) (Variables|Default|GetMinFOV) (Variables|Default|GetMaxFOV)))))

(event Input|KeyboardEvents|Backspace
  (params (Key :type Key%20Structure :default "None"))
  (bind _returnvalue (Game|GetPlayerController 0))
  (:Pressed
    (Input|DisableInput self _returnvalue)
    (Input|EnableInput (Game|GetPlayerCharacter 0) _returnvalue)
    (Transformation|SetWorldTransform (Variables|Default|GetPaper%20Mesh) (Variables|Default|GetInitial) false false)))

(fn ConstructionScript
  (Rendering|Components|TextRender|SetText (Variables|Default|GetNote%20Text) (Variables|Default|GetText))
  (Variables|Default|SetInitial (Transformation|GetWorldTransform (Variables|Default|GetPaper%20Mesh))))

(fn Lookat
  (return ""))