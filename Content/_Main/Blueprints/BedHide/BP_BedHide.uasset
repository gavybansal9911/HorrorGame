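; BP_BedHide is a bed hiding spot that lets the first-person character hide and unhide with the Hide input.
; A box overlap stores the character, enables input and opens a gate, while leaving disables input and closes it.
; Hiding blends the view to this actor, then re-enables input and reopens the gate after a short delay.
; Look input branches on the hiding state but adds only zero pitch.
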(event OnComponentBeginOverlap(Box)
  (params (OverlappedComponent :type Primitive%20Component%20Object%20Reference) (OtherActor :type Actor%20Object%20Reference) (OtherComp :type Primitive%20Component%20Object%20Reference) (OtherBodyIndex :type Integer) (bFromSweep :type Boolean) (SweepResult :type Hit%20Result%20Structure%20%28by%20ref%29))
  (bind _asbp_first_person_character (Utilities|Casting|CastToBP_FirstPersonCharacter OtherActor))
  (Variables|Default|SetCharacter%20REF _asbp_first_person_character)
  (Input|EnableInput (Game|GetPlayerController 0))
  (Utilities|FlowControl|Gate true) ; enters at Open
)

(event OnComponentEndOverlap(Box)
  (params (OverlappedComponent :type Primitive%20Component%20Object%20Reference) (OtherActor :type Actor%20Object%20Reference) (OtherComp :type Primitive%20Component%20Object%20Reference) (OtherBodyIndex :type Integer))
  (bind _returnvalue (Game|GetPlayerController 0))
  (bind _character_ref (Variables|Default|GetCharacter%20REF))
  (Utilities|Casting|CastToBP_FirstPersonCharacter OtherActor)
  (Input|DisableInput _returnvalue)
  (Utilities|FlowControl|Gate true) ; enters at Close
)

(event Input|EnhancedActionEvents|EnhancedInputActionLook
  (params (ActionValue :type Vector%202D%20Structure) (ElapsedSeconds :type Float%20%28double-precision%29) (TriggeredSeconds :type Float%20%28double-precision%29) (InputAction :type Input%20Action%20Object%20Reference :default "/Game/FirstPerson/Input/Actions/Look.Look"))
  (bind _character_ref (Variables|Default|GetCharacter%20REF))
  (:Triggered
    (if (Variables|/Game/FirstPerson/Blueprints/BP_FirstPersonCharacter.BP_FirstPersonCharacter_C|GetIsHiding? _character_ref)
      (bind _output_get (Variables|Default|SetPitch (+ (Variables|Default|GetPitch) 0.0)))
      (else
        (Pawn|Input|AddControllerPitchInput _character_ref 0.0)))))

(event Input|ActionEvents|InputActionHide
  (params (Key :type Key%20Structure))
  (bind _character_ref (Variables|Default|GetCharacter%20REF))
  (:Pressed
    (Utilities|FlowControl|Gate true :!label _label
      (:Exit
        (if (Variables|/Game/FirstPerson/Blueprints/BP_FirstPersonCharacter.BP_FirstPersonCharacter_C|GetIsHiding? _character_ref)
          (Default|UnHide _character_ref)
          (else
            (Default|Hide _character_ref)
            (Utilities|FlowControl|Sequence
              (:then_0
                (Game|Player|SetViewTargetwithBlend (Game|GetPlayerController 0) self 0.5 "VTBlend_Linear" 0.0 false))
              (:then_1
                (Utilities|FlowControl|Delay 0.2)
                (Input|EnableInput (Game|GetPlayerController 0))
                (goto _label Open)))))))))

(fn ConstructionScript)

(fn Lookat
  (return ""))