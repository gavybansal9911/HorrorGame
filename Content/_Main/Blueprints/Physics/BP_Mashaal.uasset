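; BP_Mashaal is a torch actor that can be lit and unlit, extending a parent class that provides a release hook.
; LitMashaal shows the point light and particle system and starts the audio, while UnlitMashaal hides both and stops it.
; The construction script stops the audio, and the OnRelease override runs the parent logic, then extinguishes the torch.
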(event Custom|Lit%20Mashaal
  (Rendering|SetVisibility (Variables|Default|GetPointLight) true false)
  (Audio|Components|Audio|Play (Variables|Default|GetAudio) 0.0))

(event Custom|Unlit%20Mashaal
  (Rendering|SetVisibility (Variables|Default|GetPointLight) false false)
  (Audio|Components|Audio|Stop (Variables|Default|GetAudio)))

(event EventBeginPlay
  (|CallParentFunction))

(event Collision|EventActorBeginOverlap
  (params (OtherActor :type Actor%20Object%20Reference)))

(event EventTick
  (params (DeltaSeconds :type Float%20%28single-precision%29))
  (|CallParentFunction DeltaSeconds))

(fn ConstructionScript
  (|CallParentFunction)
  (Audio|Components|Audio|Stop (Variables|Default|GetAudio)))

(fn OnRelease
  (|CallParentFunction)
  (CallFunction|UnlitMashaal))