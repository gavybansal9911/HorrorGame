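; Base actor for physics items the first-person player can pick up, carry and throw, with empty interact, look-at text and release hooks.
; Grab attaches the mesh to the player's PhysicsHandle, sets its Pawn collision to overlap and hides the item's spotlight.
; While held, Tick drives the handle target from the camera transform plus location and rotation offsets.
; Release applies a camera-forward throw impulse, drops the handle and calls OnRelease.
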(event EventBeginPlay
  (|CallParentFunction))

(event EventTick
  (params (DeltaSeconds :type Float%20%28single-precision%29))
  (bind _returnvalue (Game|GetPlayerCharacter 0))
  (bind _returnvalue_2 (Game|GetPlayerCharacter 0))
  (bind _rot_item_grab_rotation_offset (Variables|Offset|Rotation|GetRot%20Item%20Grab%20Rotation%20Offset))
  (bind (_roll _pitch _yaw) (Math|Rotator|BreakRotator _rot_item_grab_rotation_offset))
  (bind _asbp_first_person_character (Utilities|Casting|CastToBP_FirstPersonCharacter _returnvalue))
  (bind _asbp_first_person_character_2 (Utilities|Casting|CastToBP_FirstPersonCharacter _returnvalue_2))
  (bind _firstpersoncamera (Variables|/Game/FirstPerson/Blueprints/BP_FirstPersonCharacter.BP_FirstPersonCharacter_C|GetFirstPersonCamera _asbp_first_person_character_2))
  (bind _firstpersoncamera_2 (Variables|/Game/FirstPerson/Blueprints/BP_FirstPersonCharacter.BP_FirstPersonCharacter_C|GetFirstPersonCamera _asbp_first_person_character))
  (bind _returnvalue_3 (Transformation|GetWorldRotation _firstpersoncamera_2))
  (bind (_roll_2 _pitch_2 _yaw_2) (Math|Rotator|BreakRotator _returnvalue_3))
  ;[1 1 1] Item Grab Loop ( Hold )
  (if (Variables|Properties|GetIsObjectGrabbed)
    (Physics|Components|PhysicsHandle|SetTargetLocation (Variables|Default|GetPhysics%20Handle) (+ (+ (+ (Transformation|GetWorldLocation _firstpersoncamera) (* (Math|Vector|GetForwardVector _firstpersoncamera) (Variables|Offset|Location|GetLoc%20Item%20Grab%20Offset))) (* (Math|Vector|GetRightVector _firstpersoncamera) (Variables|Offset|Location|GetLoc%20Item%20Grab%20Right%20Offset))) (* (Math|Vector|GetUpVector _firstpersoncamera) (Variables|Offset|Location|GetLoc%20Item%20Grab%20Up%20Offset))))
    (Class|PhysicsHandleComponent|SetTargetRotation (Variables|Default|GetPhysics%20Handle) (Math|Rotator|MakeRotator (+ _roll_2 _roll) (+ _pitch_2 _pitch) (+ _yaw_2 _yaw)))))

(event EventInteractwith
  (params (Player%20Character :type BP%20First%20Person%20Character%20Object%20Reference) (Grabbed%20Item :type BP%20Grab%20Item%20Base%20Object%20Reference) (Hit%20Component :type Primitive%20Component%20Object%20Reference)))

(event EventGrab
  (params (Player%20Character :type BP%20First%20Person%20Character%20Object%20Reference) (Hit%20Location :type Vector :default "0, 0, 0"))
  (bind _mesh (Variables|Character|GetMesh))
  ;[1 1 1] Item Grab
  (bind _output_get (Variables|Default|SetPhysics%20Handle (Variables|/Game/FirstPerson/Blueprints/BP_FirstPersonCharacter.BP_FirstPersonCharacter_C|GetPhysicsHandle Player%20Character)))
  (Physics|Components|PhysicsHandle|GrabComponentatLocationwithRotation _output_get (Variables|Character|GetMesh) "None" (Transformation|GetWorldLocation _mesh) (Transformation|GetWorldRotation _mesh))
  (Variables|Properties|SetIsObjectGrabbed true)
  (Collision|SetCollisionResponsetoChannel (Variables|Character|GetMesh) "ECC_Pawn" "ECR_Overlap")
  (Rendering|SetVisibility (Variables|Default|GetSpotLight) false false))

(event EventRelease
  ;[1 1 1] Release
  (if (Variables|Properties|GetIsObjectGrabbed)
    (Physics|AddImpulse (Variables|Character|GetMesh) (* (Math|Vector|GetForwardVector (Variables|/Game/FirstPerson/Blueprints/BP_FirstPersonCharacter.BP_FirstPersonCharacter_C|GetFirstPersonCamera (.AsBP%20First%20Person%20Character (Utilities|Casting|CastToBP_FirstPersonCharacter (Game|GetPlayerCharacter 0))))) (Variables|Physics|GetThrow%20Force)) "None" false)
    (Physics|Components|PhysicsHandle|ReleaseComponent (Variables|Default|GetPhysics%20Handle))
    (CallFunction|OnRelease)
    (Variables|Properties|SetIsObjectGrabbed false)))

(fn ConstructionScript
  (|CallParentFunction)
  (Transformation|SetMobility (Variables|Default|GetSpotLight) "Static"))

(fn Lookat
  (return ""))

(fn OnRelease)