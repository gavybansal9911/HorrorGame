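; BP_PhysicsDoor is a door the player grabs and swings by moving the mouse.
; Grab disables player movement and look and enables the door's input, and Release restores them.
; MouseX is scaled by sensitivity and passed to MoveDoor, which adds yaw to the mesh's relative rotation without angle limits or physics simulation.
; A dot product between player-to-door direction and door forward flips the swing by side.
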(event Custom|Move%20Door
  (params (Scale :type Float%20%28double-precision%29))
  (Transformation|SetRelativeRotation (Variables|Default|GetDoor%20Mesh) (Math|Rotator|CombineRotators (Variables|/Script/Engine.SceneComponent|GetRelativeRotation (Variables|Default|GetDoor%20Mesh)) (Math|Rotator|MakeRotator 0.0 0.0 (* Scale (select (>= (Math|Vector|DotProduct (Math|Vector|Normalize (- (Transformation|GetActorLocation) (Transformation|GetActorLocation (Game|GetPlayerCharacter 0)))) (Transformation|GetActorForwardVector)) 0.0) 1.0 -1.0)))) false false))

(event EventGrab
  (bind _returnvalue (Game|GetPlayerController 0))
  (Pawn|Components|CharacterMovement|DisableMovement (Variables|/Script/Engine.Character|GetCharacterMovement (Game|GetPlayerCharacter 0)))
  (Input|SetIgnoreLookInput _returnvalue true)
  (Input|EnableInput _returnvalue))

(event EventRelease
  (bind _returnvalue (Game|GetPlayerController 0))
  (Pawn|Components|CharacterMovement|SetMovementMode (Variables|/Script/Engine.Character|GetCharacterMovement (Game|GetPlayerCharacter 0)) "MOVE_Walking" 0)
  (Input|ResetIgnoreLookInput _returnvalue)
  (Input|DisableInput _returnvalue))

(event Input|MouseEvents|MouseX
  (params (AxisValue :type Float%20%28single-precision%29))
  (CallFunction|MoveDoor (* AxisValue (Variables|Default|GetSenstivity))))

(fn ConstructionScript)