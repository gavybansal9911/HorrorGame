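; BP_Door is an interactable door that swings open and closed when the player interacts with it.
; The Interactwith event toggles IsDoorClosed and either plays or reverses the OpenDoorTL timeline.
; The timeline's alpha lerps the DoorMesh relative yaw through a quarter turn, so closing retraces the opening motion.
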(event EventBeginPlay
  (|CallParentFunction))

(event EventInteractwith
  (params (Player%20Character :type BP%20First%20Person%20Character%20Object%20Reference))
  (if (Variables|Default|GetbIsDoorClosed)
    (Variables|Default|SetbIsDoorClosed false)
    (bind _alpha (Timeline|Open%20Door%20TL Play)
      (:Update
        (Transformation|SetRelativeRotation (Variables|Default|GetDoor%20Mesh) (Math|Rotator|MakeRotator 0.0 0.0 (Math|Float|Lerp 0.0 -9e+01 _alpha)) false false)))
    (else
      (Variables|Default|SetbIsDoorClosed true)
      (Timeline|Open%20Door%20TL Reverse))))

(fn ConstructionScript
  (|CallParentFunction))