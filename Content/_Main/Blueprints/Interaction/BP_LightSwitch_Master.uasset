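; Master Blueprint for an interactable light switch that turns a referenced light on and off.
; On BeginPlay it reads the light's visibility and snaps the switch pivot to the matching on or off transform.
; Each interaction toggles the light component's visibility, plays a 2D click sound and flips the switch state.
; A single timeline, played forward or reversed, lerps the pivot's relative location and rotation between the two transforms.
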(event Custom|Turn%20On
  (Audio|PlaySound2D "/Engine/VREditor/Sounds/UI/Gizmo_Handle_Clicked.Gizmo_Handle_Clicked" 1.0 1.0 0.0 0 0)
  (Variables|Properties|SetbSwitchOn true)
  (bind _alpha (Timeline|Button%20On%20Timeline Play)
    (:Update
      (Transformation|SetRelativeLocationAndRotation (Variables|Default|GetPivot) (Math|Vector|Lerp(Vector) (Variables|Properties|GetOff%20Location) (Variables|Properties|GetOn%20Location) _alpha) (Math|Rotator|Lerp(Rotator) (Variables|Properties|GetOff%20Rotation) (Variables|Properties|GetOn%20Rotation) _alpha) false false))))

(event Custom|Turn%20Off
  (Audio|PlaySound2D "/Engine/VREditor/Sounds/UI/Gizmo_Handle_Clicked.Gizmo_Handle_Clicked" 1.0 1.0 0.0 0 0)
  (Variables|Properties|SetbSwitchOn false)
  (bind _alpha (Timeline|Button%20On%20Timeline Reverse)
    (:Update
      (Transformation|SetRelativeLocationAndRotation (Variables|Default|GetPivot) (Math|Vector|Lerp(Vector) (Variables|Properties|GetOff%20Location) (Variables|Properties|GetOn%20Location) _alpha) (Math|Rotator|Lerp(Rotator) (Variables|Properties|GetOff%20Rotation) (Variables|Properties|GetOn%20Rotation) _alpha) false false))))

(event EventBeginPlay
  (|CallParentFunction)
  (bind _output_get (Variables|Properties|SetbSwitchOn (Rendering|IsVisible (Variables|/Script/Engine.Light|GetLightComponent (Variables|Light|GetLight)))))
  (Transformation|SetRelativeLocationAndRotation (Variables|Default|GetPivot) (select _output_get (Variables|Properties|GetOn%20Location) (Variables|Properties|GetOff%20Location)) (select _output_get (Variables|Properties|GetOn%20Rotation) (Variables|Properties|GetOff%20Rotation)) false false))

(event EventInteractwith
  (params (Player%20Character :type BP%20First%20Person%20Character%20Object%20Reference))
  (bind _light (Variables|Light|GetLight))
  (bind _lightcomponent (Variables|/Script/Engine.Light|GetLightComponent _light))
  (if (Variables|Properties|GetbSwitchOn)
    (Rendering|SetVisibility _lightcomponent false false)
    (CallFunction|TurnOff)
    (else
      (Rendering|SetVisibility _lightcomponent true false)
      (CallFunction|Turnon))))

(fn ConstructionScript
  (|CallParentFunction))