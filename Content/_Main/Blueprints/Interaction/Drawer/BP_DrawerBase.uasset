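; Base Blueprint for an interactable drawer that slides open and closed when the player interacts with it.
; An unlocked drawer toggles a timeline forward or in reverse, lerping the mesh's relative location from zero along its forward vector by OpenLength.
; Interaction disables during movement and returns shortly after the timeline finishes.
; A locked drawer does not move, and its interaction stays disabled after the first attempt.
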(event EventBeginPlay
  (|CallParentFunction))

(event EventInteractwith
  (params (Player%20Character :type BP%20First%20Person%20Character%20Object%20Reference) (Grabbed%20Item :type BP%20Grab%20Item%20Base%20Object%20Reference) (Hit%20Component :type Primitive%20Component%20Object%20Reference))
  (if (Variables|Default|GetbInteractionEnabled)
    (Variables|Default|SetbInteractionEnabled false)
    (if (not (Variables|Default|GetbIsLocked))
      (if (not (Variables|Default|GetbIsOpened))
        (Variables|Default|SetbIsOpened true)
        (bind _alpha (Timeline|Drawer%20Open%20Timeline Play)
          (:Update
            (Transformation|SetRelativeLocation (Variables|Character|GetMesh) (Math|Vector|Lerp(Vector) "0, 0, 0" (* (Math|Vector|GetForwardVector (Variables|Character|GetMesh)) (Variables|Default|GetOpenLength)) _alpha) false false))
          (:Finished
            (Utilities|FlowControl|Delay 0.1)
            (Variables|Default|SetbInteractionEnabled true)))
        (else
          (Variables|Default|SetbIsOpened false)
          (Timeline|Drawer%20Open%20Timeline Reverse))))))

(fn ConstructionScript
  (|CallParentFunction))