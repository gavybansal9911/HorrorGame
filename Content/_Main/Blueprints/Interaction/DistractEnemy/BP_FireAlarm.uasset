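; BP_FireAlarm is an interactable fire alarm that the player triggers to create a loud distraction for enemies.
; Interacting plays an attenuated sound at the alarm and makes the player's ACNoise component emit a very loud, long-range noise from the alarm's location.
; Interaction is then disabled until the sound's duration plus a short buffer has passed, preventing repeated triggering.
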(event EventBeginPlay
  (|CallParentFunction))

(event EventInteractwith
  (params (Player%20Character :type BP%20First%20Person%20Character%20Object%20Reference) (Grabbed%20Item :type BP%20Grab%20Item%20Base%20Object%20Reference) (Hit%20Component :type Primitive%20Component%20Object%20Reference))
  (if (Variables|Default|GetbInteractionEnabled)
    (Variables|Default|SetbInteractionEnabled false)
    (bind _returnvalue (Audio|SpawnSoundatLocation "/Game/StarterContent/Audio/Fire_Sparks01.Fire_Sparks01" (Transformation|GetActorLocation) "0, 0, 0" 1.0 1.0 0.0 "/Game/_Main/Sounds/SA_FireAlarm.SA_FireAlarm" 0))
    (Default|MakeNoise (Variables|/Game/FirstPerson/Blueprints/BP_FirstPersonCharacter.BP_FirstPersonCharacter_C|GetAC_Noise Player%20Character) (Transformation|GetActorLocation) 1e+07 1e+08)
    (Utilities|FlowControl|Delay (+ (Variables|/Script/Engine.SoundBase|GetDuration (Variables|/Script/Engine.AudioComponent|GetSound _returnvalue)) 1.0))
    (Variables|Default|SetbInteractionEnabled true)))

(fn ConstructionScript
  (|CallParentFunction))