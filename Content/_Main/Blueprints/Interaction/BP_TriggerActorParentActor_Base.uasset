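; Base interactable Blueprint that relays a player's interaction to a referenced TriggerActor.
; When interaction is enabled and the TriggerActor implements I_TriggerInterface, it runs the OnTriggerActorFound hook, then sends OnTriggeredMessage with the player character.
; OnTriggerActorFound is an empty hook, LookAt returns an empty string, and BeginPlay and construction defer to the parent class.
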(event EventBeginPlay
  (|CallParentFunction))

(event EventInteractwith
  (params (Player%20Character :type BP%20First%20Person%20Character%20Object%20Reference))
  (if (Variables|Default|GetbInteractionEnabled)
    (if (Utilities|DoesObjectImplementInterface (Variables|Default|GetTrigger%20Actor) "/Game/_Main/Blueprints/Interfaces/I_TriggerInterface.I_TriggerInterface_C")
      (CallFunction|OnTriggerActorFound)
      (Class|ITriggerInterface|OnTriggered(Message) (Variables|Default|GetTrigger%20Actor) Player%20Character))))

(fn ConstructionScript
  (|CallParentFunction))

(fn Lookat
  (return ""))

(fn OnTriggerActorFound)