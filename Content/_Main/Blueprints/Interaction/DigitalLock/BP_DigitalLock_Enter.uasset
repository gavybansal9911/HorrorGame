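; Enter button of a digital lock that submits the entered password when the player interacts with it.
; Interacting plays a 2D press sound, then, if the referenced lock is still closed, asks it to check the password.
; A match opens the lock, while a failure resets the entered password.
; Grab and Release do nothing, and Look At returns an empty string.
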(event EventBeginPlay
  (|CallParentFunction))

(event EventRelease)

(event EventGrab
  (params (Player%20Character :type BP%20First%20Person%20Character%20Object%20Reference) (Hit%20Location :type Vector :default "0, 0, 0")))

(event EventInteractwith
  (params (Player%20Character :type BP%20First%20Person%20Character%20Object%20Reference) (Grabbed%20Item :type BP%20Grab%20Item%20Base%20Object%20Reference) (Hit%20Component :type Primitive%20Component%20Object%20Reference))
  (Audio|PlaySound2D (Variables|Default|GetOn%20Pressed%20Sound) 1.0 1.0 0.0 0 0)
  (if (not (Variables|/Game/_Main/Blueprints/Interaction/DigitalLock/BP_DigitalLock.BP_DigitalLock_C|GetIsOpened (Variables|Default|GetDigital%20Lock%20Ref)))
    (bind _correct (Default|CheckPassword (Variables|Default|GetDigital%20Lock%20Ref)))
    (if _correct
      (Default|OpenLock (Variables|Default|GetDigital%20Lock%20Ref))
      (else
        (Default|ResetEnteredPassword (Variables|Default|GetDigital%20Lock%20Ref))))))

(fn ConstructionScript
  (|CallParentFunction))

(fn Lookat
  (return ""))