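; Digital keypad lock that takes a four-digit code and, once opened, triggers or unlocks and interacts with a linked TriggerActor.
; On BeginPlay it spawns number, Enter and Reset button actors on mesh sockets, each holding a reference to the lock.
; Functions store digits, compare them to Password, open the lock or reset after a wrong-code delay.
; The display swaps textures on a dynamic material to show entry count and result.
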(event Custom|Wrong%20Password
  (bind _returnvalue (Rendering|Material|CreateDynamicMaterialInstance (Variables|Default|GetStaticMesh) 1 0 "None" :!class /Script/Engine.PrimitiveComponent))
  (Rendering|Material|SetTextureParameterValue _returnvalue "Texture" "/Game/HorrorEngine/Textures/Digit_Wrong.Digit_Wrong")
  (Audio|PlaySound2D (Variables|Sounds|GetWrong%20Password%20Sound) 1.0 1.0 0.0 0 0)
  (Utilities|FlowControl|Delay 3.0)
  (Audio|PlaySound2D "/Game/HorrorEngine/Audio/Elecronic/WrongCode_Cue.WrongCode_Cue" 1.0 1.0 0.0 0 0)
  (CallFunction|ResetEnteredPassword))

(event EventBeginPlay
  (for (_array_element _array_index) (Variables|Default|GetNumber%20Button%20Textures)
    (bind _returnvalue (Game|SpawnActorfromClass "/Game/_Main/Blueprints/Interaction/DigitalLock/BP_DigitalLock_NumberButton.BP_DigitalLock_NumberButton_C" (Math|Transform|MakeTransform "0, 0, 0" "0, 0, 0" "1.000000,1.000000,1.000000") "Undefined" "MultiplyWithRoot" 0 _array_element (Utilities|Array|Get(acopy) (Variables|Default|GetNumber%20Buttons%20Numbers) _array_index) self 0))
    (Transformation|AttachComponentToComponent _returnvalue (Variables|Default|GetStaticMesh) (Utilities|Array|Get(acopy) (Variables|Default|GetNumber%20Buttons%20Socket%20Names) _array_index) "SnapToTarget" "SnapToTarget" "SnapToTarget" true))
  (bind _returnvalue_2 (Game|SpawnActorfromClass "/Game/_Main/Blueprints/Interaction/DigitalLock/BP_DigitalLock_Enter.BP_DigitalLock_Enter_C" (Math|Transform|MakeTransform "0, 0, 0" "0, 0, 0" "1.000000,1.000000,1.000000") "Undefined" "MultiplyWithRoot" 0 self 0))
  (Transformation|AttachComponentToComponent _returnvalue_2 (Variables|Default|GetStaticMesh) "SocketEnter" "SnapToTarget" "SnapToTarget" "SnapToTarget" true)
  (bind _returnvalue_3 (Game|SpawnActorfromClass "/Game/_Main/Blueprints/Interaction/DigitalLock/BP_DigitalLock_Reset.BP_DigitalLock_Reset_C" (Math|Transform|MakeTransform "0, 0, 0" "0, 0, 0" "1.000000,1.000000,1.000000") "Undefined" "MultiplyWithRoot" 0 self 0))
  (Transformation|AttachComponentToComponent _returnvalue_3 (Variables|Default|GetStaticMesh) "SocketReset" "SnapToTarget" "SnapToTarget" "SnapToTarget" true))

(event EventInteractwith
  (params (Player%20Character :type BP%20First%20Person%20Character%20Object%20Reference) (Grabbed%20Item :type BP%20Grab%20Item%20Base%20Object%20Reference) (Hit%20Component :type Primitive%20Component%20Object%20Reference)))

(fn ConstructionScript
  (Utilities|Array|Resize (Variables|Default|GetPassword) 4)
  (Utilities|Array|Resize (Variables|Default|GetEntered%20Password) 4)
  (Rendering|Material|CreateDynamicMaterialInstance (Variables|Default|GetStaticMesh) 0 0 "None" :!class /Script/Engine.PrimitiveComponent))

(fn UpdateEnteredPassword
  (params (Number :type Integer%20%28by%20ref%29))
  (Utilities|Array|SetArrayElem (Variables|Default|GetEntered%20Password) (Variables|Default|GetCurrent%20Index) Number)
  (Math|Integer|IncrementInt (Variables|Default|GetCurrent%20Index)
    (:%20%20
      (CallFunction|UpdateDisplay))))

(fn CheckPassword
  (bind (_array_element _array_index) (Utilities|Array|ForEachLoopwithBreak (Variables|Default|GetPassword) :!label _label)
    (:LoopBody
      (Development|PrintString (Utilities|String|ToString(Integer) _array_element))
      (Development|PrintString (Utilities|String|ToString(Integer) (Utilities|Array|Get(acopy) (Variables|Default|GetEntered%20Password) _array_index)) true true "(R=0.934361,G=1.000000,B=0.000000,A=1.000000)")
      (if (== _array_element (Utilities|Array|Get(acopy) (Variables|Default|GetEntered%20Password) _array_index))
        (LocalVariables|SetLocal_Correct true)
        (else
          (Audio|PlaySound2D "/Engine/EditorSounds/Notifications/CompileFailed.CompileFailed" 1.0 1.0 0.0 0 0)
          (LocalVariables|SetLocal_Correct false)
          (goto _label Break))))
    (:Completed
      (return (LocalVariables|GetLocal_Correct)))))

(fn ResetEnteredPassword
  (bind _returnvalue (Rendering|Material|CreateDynamicMaterialInstance (Variables|Default|GetStaticMesh) 1 0 "None" :!class /Script/Engine.PrimitiveComponent))
  (Rendering|Material|SetTextureParameterValue _returnvalue "Texture" "/Game/HorrorAssets/Textures/Digit_0.Digit_0")
  (Utilities|Array|Clear (Variables|Default|GetEntered%20Password))
  (Variables|Default|SetCurrent%20Index 0)
  (Utilities|Array|Resize (Variables|Default|GetEntered%20Password) 4))

(fn UpdateDisplay
  (switch int (Variables|Default|GetCurrent%20Index)
    (:0
      (bind _returnvalue (Rendering|Material|CreateDynamicMaterialInstance (Variables|Default|GetStaticMesh) 1 0 "None" :!class /Script/Engine.PrimitiveComponent))
      (Rendering|Material|SetTextureParameterValue _returnvalue "Texture" "/Game/HorrorAssets/Textures/Digit_0.Digit_0"))
    (:1
      (bind _returnvalue_2 (Rendering|Material|CreateDynamicMaterialInstance (Variables|Default|GetStaticMesh) 1 0 "None" :!class /Script/Engine.PrimitiveComponent))
      (Rendering|Material|SetTextureParameterValue _returnvalue_2 "Texture" "/Game/HorrorEngine/Textures/Digit_1.Digit_1"))
    (:2
      (bind _returnvalue_3 (Rendering|Material|CreateDynamicMaterialInstance (Variables|Default|GetStaticMesh) 1 0 "None" :!class /Script/Engine.PrimitiveComponent))
      (Rendering|Material|SetTextureParameterValue _returnvalue_3 "Texture" "/Game/HorrorEngine/Textures/Digit_2.Digit_2"))
    (:3
      (bind _returnvalue_4 (Rendering|Material|CreateDynamicMaterialInstance (Variables|Default|GetStaticMesh) 1 0 "None" :!class /Script/Engine.PrimitiveComponent))
      (Rendering|Material|SetTextureParameterValue _returnvalue_4 "Texture" "/Game/HorrorEngine/Textures/Digit_3.Digit_3"))
    (:4
      (bind _returnvalue_5 (Rendering|Material|CreateDynamicMaterialInstance (Variables|Default|GetStaticMesh) 1 0 "None" :!class /Script/Engine.PrimitiveComponent))
      (Rendering|Material|SetTextureParameterValue _returnvalue_5 "Texture" "/Game/HorrorEngine/Textures/Digit_4.Digit_4"))))

(fn OpenLock
  (bind _player_character (CallFunction|GetMyPlayerCharacter))
  (bind _returnvalue (Rendering|Material|CreateDynamicMaterialInstance (Variables|Default|GetStaticMesh) 1 0 "None" :!class /Script/Engine.PrimitiveComponent))
  (Rendering|Material|SetTextureParameterValue _returnvalue "Texture" "/Game/HorrorEngine/Textures/Digit_Open.Digit_Open")
  (Utilities|Array|Clear (Variables|Default|GetEntered%20Password))
  (Variables|Default|SetCurrent%20Index 0)
  (Variables|Default|SetIsOpened true)
  (if (Utilities|DoesObjectImplementInterface (Variables|Default|GetTrigger%20Actor) "/Game/_Main/Blueprints/Interfaces/I_TriggerInterface.I_TriggerInterface_C")
    (Class|ITriggerInterface|OnTriggered(Message) (Variables|Default|GetTrigger%20Actor) (CallFunction|GetMyPlayerCharacter))
    (bind _asbp_interaction_actor_base (Utilities|Casting|CastToBP_InteractionActor_Base (Variables|Default|GetTrigger%20Actor) :!label _label))
    (Variables|/Game/_Main/Blueprints/Interaction/BP_InteractionActor_Base.BP_InteractionActor_Base_C|SetbLocked _asbp_interaction_actor_base false)
    (Audio|PlaySound2D "/Game/HorrorEngine/Audio/Elecronic/CorrectCode_Cue.CorrectCode_Cue" 1.0 1.0 0.0 0 0)
    (Class|IInteractInterface|Interactwith(Message) (Variables|Default|GetTrigger%20Actor) _player_character (Variables|/Game/FirstPerson/Blueprints/BP_FirstPersonCharacter.BP_FirstPersonCharacter_C|GetGrabbed%20Object _player_character))
    (elif (Utilities|DoesObjectImplementInterface (Variables|Default|GetTrigger%20Actor) "/Game/_Main/Blueprints/Interfaces/I_InteractInterface.I_InteractInterface_C")
      (goto _label))))

(fn OnTriggerActorFound
  (|CallParentFunction))