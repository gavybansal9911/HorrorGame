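; Left door of a small wardrobe that the player opens and closes by interacting, with support for being locked.
; A timeline swings the mesh's yaw toward a random 60–90 degree angle, re-rolled every update, and reverses to close.
; When locked, BP_Ward6_DoorKey unlocks it and is destroyed; anything else plays a rattle that blocks interaction until finished.
; Monk AI auto-open logic is disconnected, and the computed facing dot product is unused.
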(event OnComponentBeginOverlap(Box)
  (params (OverlappedComponent :type Primitive%20Component%20Object%20Reference) (OtherActor :type Actor%20Object%20Reference) (OtherComp :type Primitive%20Component%20Object%20Reference) (OtherBodyIndex :type Integer) (bFromSweep :type Boolean) (SweepResult :type Hit%20Result%20Structure%20%28by%20ref%29)))

(event EventBeginPlay
  (|CallParentFunction))

(event EventInteractwith
  (params (Player%20Character :type BP%20First%20Person%20Character%20Object%20Reference) (Grabbed%20Item :type BP%20Grab%20Item%20Base%20Object%20Reference) (Hit%20Component :type Primitive%20Component%20Object%20Reference))
  (if (Variables|Default|GetbInteractionEnabled)
    (if (not (Variables|Default|GetbLocked))
      (if (Variables|Default|GetbIsDoorClosed)
        (Variables|Default|SetbIsDoorClosed false)
        (Variables|Default|GetOverlapping%20Character%20Ref
          (:then
            (bind _alpha (Timeline|Open%20Door%20TL Play)
              (:Update
                (Transformation|SetRelativeRotation (Variables|Default|GetDoor%20Mesh) (Math|Rotator|MakeRotator 0.0 0.0 (Math|Float|Lerp 0.0 (Math|Random|RandomFloatinRange 6e+01 9e+01) _alpha)) false false))))
          (:else
            (Variables|Default|SetDot%20Product (Math|Vector|DotProduct (Math|Vector|Normalize (- (Transformation|GetActorLocation) (Transformation|GetActorLocation (Variables|Default|GetPlayer%20Ref)))) (Transformation|GetActorForwardVector)))
            (Timeline|Open%20Door%20TL Play)))
        (else
          (Variables|Default|SetbIsDoorClosed true)
          (Timeline|Open%20Door%20TL Reverse)))
      (else
        (bind _asbp_ward_6_door_key (Utilities|Casting|CastToBP_Ward6_DoorKey Grabbed%20Item)
          (:then
            (Variables|Default|SetbLocked false)
            (Variables|/Game/FirstPerson/Blueprints/BP_FirstPersonCharacter.BP_FirstPersonCharacter_C|SetGrabbed%20Object Player%20Character 0)
            (Actor|DestroyActor _asbp_ward_6_door_key))
          (:CastFailed
            (Variables|Default|SetbInteractionEnabled false)
            (bind _alpha_2 (Timeline|Timeline PlayFromStart)
              (:Update
                (Transformation|SetRelativeRotation (Variables|Default|GetDoor%20Mesh) (Math|Rotator|MakeRotator 0.0 0.0 (Math|Float|Lerp 0.0 (Variables|Default|GetLockedDoorMovementRange) _alpha_2)) false false))
              (:Finished
                (Variables|Default|SetbInteractionEnabled true)))))))))

(fn ConstructionScript
  (|CallParentFunction))