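; BP_TakeOutBasementPotalDoor1 is an interactable door that acts as a portal, apparently taking the player out of the basement.
; On interaction, if interaction is enabled and the door is unlocked, it shows the WBP_AreaChangeLoadScreen widget.
; It then immediately moves the player character to a hard-coded location and rotation, with no level load.
; BeginPlay and the construction script only call their parent versions.
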(event EventBeginPlay
  (|CallParentFunction))

(event EventInteractwith
  (params (Player%20Character :type BP%20First%20Person%20Character%20Object%20Reference) (Grabbed%20Item :type BP%20Grab%20Item%20Base%20Object%20Reference) (Hit%20Component :type Primitive%20Component%20Object%20Reference))
  (bind _returnvalue (Game|GetPlayerCharacter 0))
  (if (Variables|Default|GetbInteractionEnabled)
    (if (not (Variables|Default|GetbLocked))
      (bind _returnvalue_2 (UserInterface|CreateWidget "/Game/_Main/UI/WBP_AreaChangeLoadScreen.WBP_AreaChangeLoadScreen_C"))
      (UserInterface|Viewport|AddtoViewport _returnvalue_2 0)
      (Transformation|SetActorLocation _returnvalue "295.000000,-840.000000,200.000000" false false)
      (Transformation|SetActorRotation _returnvalue))))

(fn ConstructionScript
  (|CallParentFunction))