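; BP_OutDoor is an interactable swinging door that toggles open and closed when interacted with while interaction is enabled.
; On opening, it dots the player-to-door direction with the door's forward vector to pick a positive or negative 90-degree yaw based on the player's side.
; A timeline lerps the door mesh's relative yaw to that angle and plays in reverse to close it.
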(event EventBeginPlay
  (|CallParentFunction))

(event EventInteractwith
  (params (Player%20Character :type BP%20First%20Person%20Character%20Object%20Reference) (Grabbed%20Item :type BP%20Grab%20Item%20Base%20Object%20Reference) (Hit%20Component :type Primitive%20Component%20Object%20Reference))
  (if (Variables|Default|GetbInteractionEnabled)
    (if (Variables|Default|GetbIsDoorClosed)
      (Variables|Default|SetbIsDoorClosed false)
      (Variables|Default|SetDot%20Product (Math|Vector|DotProduct (Math|Vector|Normalize (- (Transformation|GetActorLocation) (Transformation|GetActorLocation (Variables|Default|GetPlayer%20Ref)))) (Transformation|GetActorForwardVector)))
      (bind _alpha (Timeline|Open%20Door%20TL Play)
        (:Update
          (Transformation|SetRelativeRotation (Variables|Default|GetDoor%20Mesh) (Math|Rotator|MakeRotator 0.0 0.0 (Math|Float|Lerp 0.0 (Math|Float|SelectFloat 9e+01 -9e+01 (>= (Variables|Default|GetDot%20Product) 0.0)) _alpha)) false false)))
      (else
        (Variables|Default|SetbIsDoorClosed true)
        (Timeline|Open%20Door%20TL Reverse)))))

(fn ConstructionScript
  (|CallParentFunction))