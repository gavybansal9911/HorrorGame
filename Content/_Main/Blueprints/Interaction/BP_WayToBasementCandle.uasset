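; BP_WayToBasementCandle is an interactable candle that, when lit with a matchbox, sends the player to a fixed spot, by its name the basement.
; Interacting while lit puts it out; interacting while unlit requires a BP_MatchBox as the grabbed item.
; Lighting shows the point light and flame material cached at construction, then after short delays displays an area-change loading screen, moves and rotates the player, and later extinguishes itself.
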(event EventRelease)

(event EventGrab
  (params (Player%20Character :type BP%20First%20Person%20Character%20Object%20Reference) (Hit%20Location :type Vector :default "0, 0, 0")))

(event EventInteractwith
  (params (Player%20Character :type BP%20First%20Person%20Character%20Object%20Reference) (Grabbed%20Item :type BP%20Grab%20Item%20Base%20Object%20Reference) (Hit%20Component :type Primitive%20Component%20Object%20Reference))
  (bind _returnvalue (Game|GetPlayerCharacter 0))
  (if (Rendering|IsVisible (Variables|Default|GetPointLight))
    (Rendering|SetVisibility (Variables|Default|GetPointLight) false false)
    (Rendering|Material|SetMaterial (Variables|Character|GetMesh) 1 "/Game/_Main/Materials/M_Transparent.M_Transparent")
    (else
      (Utilities|Casting|CastToBP_MatchBox Grabbed%20Item)
      (Rendering|SetVisibility (Variables|Default|GetPointLight) true false)
      (Rendering|Material|SetMaterial (Variables|Character|GetMesh) 1 (Variables|Default|GetCandle%20Flame%20Material))
      (Utilities|FlowControl|Delay 0.45)
      (bind _returnvalue_2 (UserInterface|CreateWidget "/Game/_Main/UI/WBP_AreaChangeLoadScreen.WBP_AreaChangeLoadScreen_C"))
      (UserInterface|Viewport|AddtoViewport _returnvalue_2 0)
      (Transformation|SetActorLocation _returnvalue "2321.000000,640.000000,-232.000000" false false)
      (Transformation|SetActorRotation _returnvalue "0.000000,-90.000000,0.000000")
      (Utilities|FlowControl|Delay 2.5)
      (Rendering|SetVisibility (Variables|Default|GetPointLight) false false)
      (Rendering|Material|SetMaterial (Variables|Character|GetMesh) 1 "/Game/_Main/Materials/M_Transparent.M_Transparent"))))

(fn ConstructionScript
  (Variables|Default|SetCandle%20Flame%20Material (Rendering|Material|GetMaterial (Variables|Character|GetMesh) 1)))