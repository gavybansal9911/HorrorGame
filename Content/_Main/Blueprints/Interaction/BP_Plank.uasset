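; BP_Plank is an interactable wooden plank that the player knocks loose with a hammer.
; When interacted with while holding a BP_Hammer, it plays a hit sound, enables physics on its mesh, lets pawns overlap it and disables further interaction.
; Any other held item shows a "Need a Hammer" notification widget and briefly locks interaction through a delay before re-enabling it.
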(event EventBeginPlay
  (|CallParentFunction))

(event EventInteractwith
  (params (Player%20Character :type BP%20First%20Person%20Character%20Object%20Reference) (Grabbed%20Item :type BP%20Grab%20Item%20Base%20Object%20Reference) (Hit%20Component :type Primitive%20Component%20Object%20Reference))
  (if (Variables|Default|GetbInteractionEnabled)
    (Utilities|Casting|CastToBP_Hammer Grabbed%20Item
      (:then
        (Audio|PlaySoundatLocation "/Game/_Main/Sounds/SFX/SFX_WoodHitHammer.SFX_WoodHitHammer" (Transformation|GetActorLocation) "0, 0, 0" 1.0 1.0 0.0 0 0 0 0)
        (Physics|SetSimulatePhysics (Variables|Character|GetMesh) true)
        (Collision|SetCollisionResponsetoChannel (Variables|Character|GetMesh) "ECC_Pawn" "ECR_Overlap")
        (Variables|Default|SetbInteractionEnabled false))
      (:CastFailed
        (bind _returnvalue (UserInterface|CreateWidget "/Game/_Main/UI/W_NotifyPlayerUI.W_NotifyPlayerUI_C" 0 "Need a Hammer"))
        (UserInterface|Viewport|AddtoViewport _returnvalue 0)
        (Variables|Default|SetbInteractionEnabled false)
        (Utilities|FlowControl|Delay 3.4)
        (Variables|Default|SetbInteractionEnabled true)))))

(fn ConstructionScript
  (|CallParentFunction))