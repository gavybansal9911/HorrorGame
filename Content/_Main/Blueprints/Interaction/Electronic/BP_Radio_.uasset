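; BP_Radio_ is an interactable electronic radio that plays attached audio when turned on and shows a point light while it is on.
; Each interaction stops the current audio, defers to the parent's interaction logic, then syncs the light to IsOn.
; An optional looping timer auto-interacts on the player's behalf.
; An interaction with a valid hit component disables this mode, and the timer clears itself after its next firing.
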(event Custom|Interact%20With%20Timer%20Event
  (bind _returnvalue (Game|GetPlayerCharacter 0))
  (bind _asbp_first_person_character (Utilities|Casting|CastToBP_FirstPersonCharacter _returnvalue))
  (CallFunction|Interactwith _asbp_first_person_character (Variables|/Game/FirstPerson/Blueprints/BP_FirstPersonCharacter.BP_FirstPersonCharacter_C|GetGrabbed%20Object _asbp_first_person_character))
  (if (not (Variables|Default|GetAuto%20Turn%20On/Off))
    (Utilities|Time|ClearandInvalidateTimerbyHandle (stale EventBeginPlay _returnvalue))))

(event EventBeginPlay
  (|CallParentFunction)
  (if (Variables|Default|GetAuto%20Turn%20On/Off)
    (bind _returnvalue (Utilities|Time|SetTimerbyEvent (delegate Custom|Interact%20With%20Timer%20Event) (Variables|Default|GetAuto%20Turn%20On/Off%20Loop%20Time) true))))

(event EventInteractwith
  (params (Player%20Character :type BP%20First%20Person%20Character%20Object%20Reference) (Grabbed%20Item :type BP%20Grab%20Item%20Base%20Object%20Reference) (Hit%20Component :type Primitive%20Component%20Object%20Reference))
  (bind _audio_component_ref (Variables|Default|GetAudio%20Component%20Ref))
  (Utilities|IsValid _audio_component_ref
    (:Is%20Valid
      (Audio|Components|Audio|Stop _audio_component_ref))
    (:Is%20Not%20Valid
      _))
  (|CallParentFunction Player%20Character Grabbed%20Item Hit%20Component)
  (if (Variables|Default|GetbIsOn)
    (Rendering|SetVisibility (Variables|Default|GetPointLight) true false)
    (else
      (Rendering|SetVisibility (Variables|Default|GetPointLight) false false)))
  (Utilities|IsValid Hit%20Component
    (:Is%20Valid
      (Variables|Default|SetAuto%20Turn%20On/Off false))))

(fn ConstructionScript
  (|CallParentFunction)
  (Rendering|Components|Light|SetIntensity (Variables|Default|GetPointLight) (Variables|Default|GetLight%20Intensity)))

(fn OnTurnedon
  (bind _audio_component_ref (CallFunction|SpawnSound (Variables|Sounds|GetRadio%20Audio) (Variables|Character|GetMesh) (Transformation|GetActorLocation) (Variables|Default|GetStart%20Time)))
  (Variables|Default|SetAudio%20Component%20Ref _audio_component_ref)
  (return))

(fn OnTurnedOff
  (Development|PrintString "Radio Turned Off!" true true "(R=1.000000,G=0.488418,B=0.000000,A=1.000000)")
  (|CallParentFunction))