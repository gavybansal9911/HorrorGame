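; Base Blueprint for interactable electronic items that the player switches on and off.
; Interacting runs On / Off, which flips IsOn, plays the matching attached sound and makes an effectively unlimited-range noise through the player's ACNoise component.
; Interaction stays locked for the sound's duration, shortened by an offset when turning on, before the empty OnTurnedOn or OnTurnedOff hook is called.
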(event EventBeginPlay
  (|CallParentFunction))

(event EventInteractwith
  (params (Player%20Character :type BP%20First%20Person%20Character%20Object%20Reference) (Grabbed%20Item :type BP%20Grab%20Item%20Base%20Object%20Reference) (Hit%20Component :type Primitive%20Component%20Object%20Reference))
  (if (Variables|Default|GetbInteractionEnabled)
    (Utilities|On/Off)))

(fn ConstructionScript
  (|CallParentFunction))

(fn Lookat
  (return ""))

(fn SpawnSound
  (params (Sound :type Sound%20Base%20Object%20Reference) (AttachToComponent :type Scene%20Component%20Object%20Reference) (Location :type Vector) (StartTime :type Float%20%28single-precision%29) (AttenuationSettings :type Sound%20Attenuation%20Object%20Reference))
  (bind _returnvalue (Audio|SpawnSoundAttached Sound AttachToComponent "None" Location "0, 0, 0" "KeepRelativeOffset" true 1.0 1.0 StartTime AttenuationSettings 0))
  (return (Variables|/Script/Engine.SoundBase|GetDuration (Variables|/Script/Engine.AudioComponent|GetSound _returnvalue)) _returnvalue))

(fn OnTurnedon
  (return))

(fn OnTurnedOff)