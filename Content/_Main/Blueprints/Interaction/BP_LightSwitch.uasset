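; BP_LightSwitch is an interactable switch that turns a referenced light on and off.
; Its Interactwith event checks whether that light's LightComponent is visible and sets the opposite visibility, without propagating to child components.
; BeginPlay and the construction script only call their parent implementations.
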(event EventBeginPlay
  (|CallParentFunction))

(event EventInteractwith
  (params (Player%20Character :type BP%20First%20Person%20Character%20Object%20Reference))
  (bind _light (Variables|Default|GetLight))
  (bind _lightcomponent (Variables|/Script/Engine.Light|GetLightComponent _light))
  (if (Rendering|IsVisible (Variables|/Script/Engine.Light|GetLightComponent (Variables|Default|GetLight)))
    (Rendering|SetVisibility _lightcomponent false false)
    (else
      (Rendering|SetVisibility _lightcomponent true false))))

(fn ConstructionScript
  (|CallParentFunction))