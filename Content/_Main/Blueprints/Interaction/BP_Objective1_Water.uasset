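; Interactable water pickup that serves as an objective step, likely the first, and restores the player's thirst.
; On interaction it plays a 2D sound and adds a fixed amount to the player's Thirst, clamped to MaxThirst.
; It then completes the current objective through the player's objective system component, assigns NextObjective, and destroys itself.
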(event EventBeginPlay
  (|CallParentFunction))

(event EventInteractwith
  (params (Player%20Character :type BP%20First%20Person%20Character%20Object%20Reference) (Grabbed%20Item :type BP%20Grab%20Item%20Base%20Object%20Reference) (Hit%20Component :type Primitive%20Component%20Object%20Reference))
  (bind _ac_objectivesystem (Variables|/Game/FirstPerson/Blueprints/BP_FirstPersonCharacter.BP_FirstPersonCharacter_C|GetAC_ObjectiveSystem Player%20Character))
  ;[1 1 1] Water Drink sound
  (Audio|PlaySound2D 0 1.0 1.0 0.0 0 0)
  (Variables|/Game/FirstPerson/Blueprints/BP_FirstPersonCharacter.BP_FirstPersonCharacter_C|SetThirst Player%20Character (Math|Float|Clamp(Float) (+ (Variables|/Game/FirstPerson/Blueprints/BP_FirstPersonCharacter.BP_FirstPersonCharacter_C|GetThirst Player%20Character) 1e+02) 0.0 (Variables|/Game/FirstPerson/Blueprints/BP_FirstPersonCharacter.BP_FirstPersonCharacter_C|GetMaxThirst Player%20Character)))
  (Default|CompleteObjective _ac_objectivesystem)
  (Default|AssignNewObjective _ac_objectivesystem (Variables|Default|GetNext%20Objective))
  (Actor|DestroyActor))

(fn ConstructionScript
  (|CallParentFunction))