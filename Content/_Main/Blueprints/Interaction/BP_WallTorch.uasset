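; Interactable wall torch that toggles between lit and unlit, switching its particle effect, point light and audio together.
; Interact checks particle and light visibility to choose the state, then restores default intensity and briefly locks interaction with a delay.
; Lighting also plays a one-shot ignition sound at the flame.
; Separate FlickerOn/FlickerOff events drive a timeline that scales the light's current intensity each update.
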(event Custom|Lit%20Torch
  (Audio|Components|Audio|Play (Variables|Default|GetAudio) 0.0)
  (Rendering|SetVisibility (Variables|Default|GetParticleSystem) true false)
  (Rendering|SetVisibility (Variables|Default|GetPointLight) true false)
  (Audio|SpawnSoundatLocation "/Game/HorrorEngine/Audio/LighterAndTorch/LitTorch.LitTorch" (Transformation|GetWorldLocation (Variables|Default|GetParticleSystem)) "0, 0, 0" 1.0 1.0 0.0 0 0)
  (Rendering|Components|Light|SetIntensity (Variables|Default|GetPointLight) (Variables|Default|GetDefault%20Intensity))
  (Variables|Default|SetbInteractionEnabled false)
  (Utilities|FlowControl|Delay 0.75)
  (Variables|Default|SetbInteractionEnabled true))

(event Custom|Unlit%20Torch
  (Audio|Components|Audio|Stop (Variables|Default|GetAudio))
  (Rendering|SetVisibility (Variables|Default|GetParticleSystem) false false)
  (Rendering|SetVisibility (Variables|Default|GetPointLight) false false)
  (Rendering|Components|Light|SetIntensity (Variables|Default|GetPointLight) (Variables|Default|GetDefault%20Intensity))
  (Variables|Default|SetbInteractionEnabled false)
  (Utilities|FlowControl|Delay 0.75)
  (Variables|Default|SetbInteractionEnabled true))

(event Custom|FlickerOff
  (bind _attenuation (Timeline|Timeline Stop)
    (:Update
      (Rendering|Components|Light|SetIntensity (Variables|Default|GetPointLight) (* _attenuation (Variables|/Script/Engine.LightComponentBase|GetIntensity (Variables|Default|GetPointLight)))))))

(event Custom|FlickerOn
  (bind _attenuation (Timeline|Timeline Play)
    (:Update
      (Rendering|Components|Light|SetIntensity (Variables|Default|GetPointLight) (* _attenuation (Variables|/Script/Engine.LightComponentBase|GetIntensity (Variables|Default|GetPointLight)))))))

(event EventBeginPlay
  (|CallParentFunction)
  (Audio|SpawnSoundAttached 0 0 "None" "0, 0, 0" "0, 0, 0" "KeepRelativeOffset" false 1.0 1.0 0.0 0 0 false)
  (Variables|Default|SetDefault%20Intensity (Variables|/Script/Engine.LightComponentBase|GetIntensity (Variables|Default|GetPointLight))))

(event EventInteractwith
  (params (Player%20Character :type BP%20First%20Person%20Character%20Object%20Reference) (Grabbed%20Item :type BP%20Grab%20Item%20Base%20Object%20Reference) (Hit%20Component :type Primitive%20Component%20Object%20Reference))
  (if (Variables|Default|GetbInteractionEnabled)
    (if (and (Variables|/Script/Engine.SceneComponent|GetbVisible (Variables|Default|GetParticleSystem)) (Variables|/Script/Engine.SceneComponent|GetbVisible (Variables|Default|GetPointLight)))
      (CallFunction|UnlitTorch)
      (else
        (CallFunction|LitTorch)))))

(fn ConstructionScript
  (|CallParentFunction))