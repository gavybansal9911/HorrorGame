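; BP_DigitalLock is an interactable keypad lock with digit buttons 0 to 9 plus Enter and Reset, still in skeleton form.
; Interactwith compares the hit component against each button in a branch chain, and every match calls the same ButtonTimeline event.
; ButtonTimeline, Grab and Release are empty and Look At returns an empty string, so no code entry or unlock logic exists yet.
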(event Custom|Button%20Timeline)

(event EventBeginPlay
  (|CallParentFunction))

(event EventInteractwith
  (params (Player%20Character :type BP%20First%20Person%20Character%20Object%20Reference) (Grabbed%20Item :type BP%20Grab%20Item%20Base%20Object%20Reference) (Hit%20Component :type Primitive%20Component%20Object%20Reference))
  (if (== Hit%20Component (Variables|Default|GetButton0))
    (CallFunction|ButtonTimeline :!label _label)
    (elif (== Hit%20Component (Variables|Default|GetButton1))
      (goto _label)
      (elif (== Hit%20Component (Variables|Default|GetButton2))
        (goto _label)
        (elif (== Hit%20Component (Variables|Default|GetButton3))
          (goto _label)
          (elif (== Hit%20Component (Variables|Default|GetButton4))
            (goto _label)
            (elif (== Hit%20Component (Variables|Default|GetButton5))
              (goto _label)
              (elif (== Hit%20Component (Variables|Default|GetButton6))
                (goto _label)
                (elif (== Hit%20Component (Variables|Default|GetButton7))
                  (goto _label)
                  (elif (== Hit%20Component (Variables|Default|GetButton8))
                    (goto _label)
                    (elif (== Hit%20Component (Variables|Default|GetButton9))
                      (goto _label)
                      (elif (== Hit%20Component (Variables|Default|GetButtonEnter))
                        (goto _label)
                        (elif (== Hit%20Component (Variables|Default|GetButtonReset))
                          (goto _label))))))))))))))

(event EventRelease)

(event EventGrab
  (params (Player%20Character :type BP%20First%20Person%20Character%20Object%20Reference) (Hit%20Location :type Vector :default "0, 0, 0")))

(fn ConstructionScript
  (|CallParentFunction))

(fn Lookat
  (return ""))