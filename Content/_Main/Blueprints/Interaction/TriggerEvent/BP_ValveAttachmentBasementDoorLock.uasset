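; Valve attachment point for a basement door lock that the player fits with a carried valve and then operates to unlock.
; The first interaction accepts only a BP_Valve, disables its physics, snaps it to the ValveSocket and clears the player's grabbed object.
; Once the valve is attached, interactions run the parent's interact logic and then clear the Locked flag.
; A valve rotation timeline exists but is not wired to run.
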(event EventInteractwith
  (params (Player%20Character :type BP%20First%20Person%20Character%20Object%20Reference) (Grabbed%20Item :type BP%20Grab%20Item%20Base%20Object%20Reference) (Hit%20Component :type Primitive%20Component%20Object%20Reference))
  (bind _mesh (Variables|Character|GetMesh))
  (bind _base_mesh (Variables|/Game/_Main/Blueprints/Interaction/BP_InteractionActor_Base.BP_InteractionActor_Base_C|GetBase%20Mesh Grabbed%20Item))
  (if (not (Variables|Default|GetbIsValveAttached))
    (Utilities|Casting|CastToBP_Valve Grabbed%20Item)
    (Physics|SetSimulatePhysics (Variables|/Game/_Main/Blueprints/Interaction/BP_InteractionActor_Base.BP_InteractionActor_Base_C|GetMesh Grabbed%20Item) false)
    (Transformation|AttachActorToActor Grabbed%20Item self "ValveSocket" "SnapToTarget" "SnapToTarget" "SnapToTarget" true)
    (Transformation|SetWorldLocation _base_mesh (Transformation|GetSocketLocation _mesh "ValveSocket") false false)
    (Transformation|SetWorldRotation _base_mesh (Transformation|GetSocketRotation _mesh "ValveSocket") false false)
    (Variables|/Game/FirstPerson/Blueprints/BP_FirstPersonCharacter.BP_FirstPersonCharacter_C|SetGrabbed%20Object Player%20Character 0)
    (Variables|Default|SetbIsValveAttached true)
    (else
      (|CallParentFunction Player%20Character Grabbed%20Item Hit%20Component)
      (Variables|Default|SetbLocked false))))

(fn ConstructionScript
  (|CallParentFunction))