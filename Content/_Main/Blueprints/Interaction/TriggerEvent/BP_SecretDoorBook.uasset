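; BP_SecretDoorBook is an interactable book, named for a secret door, that tilts when triggered.
; Its trigger-found override calls MoveBook, then hands off to the parent logic.
; MoveBook disables interaction and toggles IsInPlace, playing a timeline forward or in reverse to pitch the mesh between level and -45 degrees on yaw.
; Interaction re-enables one second after the timeline finishes.
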(event Custom|Move%20Book
  (Variables|Default|SetbInteractionEnabled false)
  (if (Variables|Default|GetbIsInPlace)
    (Variables|Default|SetbIsInPlace false)
    (bind _alpha (Timeline|Move%20Book%20Timeline Play)
      (:Update
        (Transformation|SetRelativeRotation (Variables|Character|GetMesh) (Math|Rotator|MakeRotator 0.0 0.0 (Math|Float|Lerp 0.0 -45.0 _alpha)) false false))
      (:Finished
        (Utilities|FlowControl|Delay 1.0)
        (Variables|Default|SetbInteractionEnabled true)))
    (else
      (Variables|Default|SetbIsInPlace true)
      (Timeline|Move%20Book%20Timeline Reverse))))

(event EventBeginPlay
  (|CallParentFunction))

(fn ConstructionScript
  (|CallParentFunction))

(fn OnTriggerActorFound
  (CallFunction|MoveBook)
  (|CallParentFunction))