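; Photo evidence pickup that the player collects during the "Find Evidences" objective.
; On interaction it increments the player's AC_ObjectiveSystem progress and UI counter if that objective is active, then plays a sound and destroys itself.
; The tenth pickup instead completes the objective, assigns "Escape the Hospital", and destroys itself without the sound.
; The construction script applies each instance's photo texture through a dynamic material instance.
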(event EventBeginPlay
  (|CallParentFunction))

(event EventInteractwith
  (params (Player%20Character :type BP%20First%20Person%20Character%20Object%20Reference) (Grabbed%20Item :type BP%20Grab%20Item%20Base%20Object%20Reference) (Hit%20Component :type Primitive%20Component%20Object%20Reference))
  (bind _returnvalue (Actor|GetComponentbyClass Player%20Character "/Game/_Main/Blueprints/Components/AC_ObjectiveSystem.AC_ObjectiveSystem_C"))
  (bind _current_objective_progress (Variables|/Game/_Main/Blueprints/Components/AC_ObjectiveSystem.AC_ObjectiveSystem_C|GetCurrent%20Objective%20Progress _returnvalue))
  (Utilities|IsValid _returnvalue
    (:Is%20Valid
      (if (== (.objectiveindex (Default|GetCurrentObjective _returnvalue)) 1)
        (Math|Integer|IncrementInt _current_objective_progress
          (:%20%20
            (Default|UpdateUIText _returnvalue (Utilities|Text|FormatText "{Name} {Progress}{Separator}{ProgressOutOf}" (Utilities|Text|MakeLiteralText "Find Evidences") (Variables|/Game/_Main/Blueprints/Components/AC_ObjectiveSystem.AC_ObjectiveSystem_C|GetCurrent%20Objective%20Progress _returnvalue) (Utilities|Text|MakeLiteralText "/") (Utilities|Text|MakeLiteralText "10")))
            (if (== _current_objective_progress 10)
              (Default|CompleteObjective _returnvalue)
              (Default|AssignNewObjective _returnvalue (Utilities|Struct|MakeFObjectiveData "Escape the Hospital" 2))
              (Actor|DestroyActor)
              (else
                (Audio|PlaySound2D "/Engine/VREditor/Sounds/UI/Object_Snaps_To_Another_Actor.Object_Snaps_To_Another_Actor" 1.0 1.0 0.0 0 0)
                (Actor|DestroyActor)))))))))

(fn ConstructionScript
  (bind _returnvalue (Rendering|Material|CreateDynamicMaterialInstance (Variables|Character|GetMesh) 0 (Rendering|Material|GetMaterial (Variables|Character|GetMesh) 0) "None" :!class /Script/Engine.PrimitiveComponent))
  (Rendering|Material|SetTextureParameterValue _returnvalue "Photo Texture" (Variables|Default|GetPhoto%20Texture))
  (|CallParentFunction))