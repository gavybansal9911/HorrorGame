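; Interactable candle that the player lights with a held BP_Lighter and puts out with or without one.
; Interactwith and OnTriggered share the same toggle, checking the passed item or the player's grabbed object for the lighter.
; The point light's visibility serves as the lit state, with the flame material slot swapped to transparent when out.
; The construction script caches the original flame material and sets the light's mobility to Static.
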(event EventOff)

(event EventOn)

(event EventRelease)

(event EventGrab
  (params (Player%20Character :type BP%20First%20Person%20Character%20Object%20Reference) (Hit%20Location :type Vector :default "0, 0, 0")))

(event EventInteractwith
  (params (Player%20Character :type BP%20First%20Person%20Character%20Object%20Reference) (Grabbed%20Item :type BP%20Grab%20Item%20Base%20Object%20Reference) (Hit%20Component :type Primitive%20Component%20Object%20Reference))
  (if (Rendering|IsVisible (Variables|Default|GetPointLight))
    (Rendering|SetVisibility (Variables|Default|GetPointLight) false false)
    (Rendering|Material|SetMaterial (Variables|Character|GetMesh) 1 "/Game/_Main/Materials/M_Transparent.M_Transparent")
    (else
      (Utilities|Casting|CastToBP_Lighter Grabbed%20Item)
      (Rendering|SetVisibility (Variables|Default|GetPointLight) true false)
      (Rendering|Material|SetMaterial (Variables|Character|GetMesh) 1 (Variables|Default|GetCandle%20Flame%20Material)))))

(event EventOnTriggered
  (params (Player%20Character :type BP%20First%20Person%20Character%20Object%20Reference))
  (if (Rendering|IsVisible (Variables|Default|GetPointLight))
    (Rendering|SetVisibility (Variables|Default|GetPointLight) false false)
    (Rendering|Material|SetMaterial (Variables|Character|GetMesh) 1 "/Game/_Main/Materials/M_Transparent.M_Transparent")
    (else
      (Utilities|Casting|CastToBP_Lighter (Variables|/Game/FirstPerson/Blueprints/BP_FirstPersonCharacter.BP_FirstPersonCharacter_C|GetGrabbed%20Object Player%20Character))
      (Rendering|SetVisibility (Variables|Default|GetPointLight) true false)
      (Rendering|Material|SetMaterial (Variables|Character|GetMesh) 1 (Variables|Default|GetCandle%20Flame%20Material)))))

(fn ConstructionScript
  (Variables|Default|SetCandle%20Flame%20Material (Rendering|Material|GetMaterial (Variables|Character|GetMesh) 1))
  (Transformation|SetMobility (Variables|Default|GetPointLight) "Static"))

(fn Lookat
  (return ""))