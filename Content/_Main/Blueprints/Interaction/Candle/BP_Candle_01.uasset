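; BP_Candle_01 is an interactable candle that can be put out.
; Interactwith hides the visible PointLight and swaps the mesh's flame material slot to M_Transparent, with no path to relight it.
; The construction script caches the original flame material in CandleFlameMaterial, which the event graph never uses.
; The Grab and Release events are empty.
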(event EventInteractwith
  (params (Player%20Character :type BP%20First%20Person%20Character%20Object%20Reference) (Grabbed%20Item :type BP%20Grab%20Item%20Base%20Object%20Reference) (Hit%20Component :type Primitive%20Component%20Object%20Reference))
  (if (Rendering|IsVisible (Variables|Default|GetPointLight))
    (Rendering|SetVisibility (Variables|Default|GetPointLight) false false)
    (Rendering|Material|SetMaterial (Variables|Character|GetMesh) 1 "/Game/_Main/Materials/M_Transparent.M_Transparent")))

(event EventRelease)

(event EventGrab
  (params (Player%20Character :type BP%20First%20Person%20Character%20Object%20Reference) (Hit%20Location :type Vector :default "0, 0, 0")))

(fn ConstructionScript
  (Variables|Default|SetCandle%20Flame%20Material (Rendering|Material|GetMaterial (Variables|Character|GetMesh) 1)))