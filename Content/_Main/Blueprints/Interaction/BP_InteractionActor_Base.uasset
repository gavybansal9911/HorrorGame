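; BP_InteractionActor_Base is a base actor for objects the first-person player can interact with.
; On BeginPlay it caches the player's BP_FirstPersonCharacter and, if that cast succeeds, applies its own custom time dilation setting.
; The Interactwith event only prints a debug message when interaction is enabled, while OnTrigger is an empty stub and LookAt returns an empty string.
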(event EventBeginPlay
  (bind _asbp_first_person_character (Utilities|Casting|CastToBP_FirstPersonCharacter (Game|GetPlayerCharacter 0)))
  (Variables|Ref|SetPlayer%20Ref _asbp_first_person_character)
  (Variables|Default|SetCustomTimeDilation (Variables|Default|GetCustom%20Time%20Dialation)))

(event EventInteractwith
  (params (Player%20Character :type BP%20First%20Person%20Character%20Object%20Reference) (Grabbed%20Item :type BP%20Grab%20Item%20Base%20Object%20Reference) (Hit%20Component :type Primitive%20Component%20Object%20Reference))
  (if (Variables|Interaction|GetbInteractionEnabled)
    (Development|PrintString "Interact Actor Base!")))

(fn ConstructionScript)

(fn OnTrigger)

(fn Lookat
  (return ""))