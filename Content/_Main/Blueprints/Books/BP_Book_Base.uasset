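; Base Blueprint for readable books that open a reading screen when the player interacts with them.
; If interaction is enabled, Interactwith pauses the game and creates a W_BookReadWidget fed by the book's BookData.
; It then adds the widget to the viewport, switches the first player controller to UI-only input and shows the mouse cursor.
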(event EventBeginPlay
  (|CallParentFunction))

(event EventInteractwith
  (params (Player%20Character :type BP%20First%20Person%20Character%20Object%20Reference) (Grabbed%20Item :type BP%20Grab%20Item%20Base%20Object%20Reference) (Hit%20Component :type Primitive%20Component%20Object%20Reference))
  (if (Variables|Default|GetbInteractionEnabled)
    (Game|SetGamePaused true)
    (bind _returnvalue (UserInterface|CreateWidget "/Game/_Main/UI/W_BookReadWidget.W_BookReadWidget_C" 0 (Variables|Default|GetBookData)))
    (UserInterface|Viewport|AddtoViewport _returnvalue 0)
    (Input|SetInputModeUIOnly (Game|GetPlayerController 0) 0 "DoNotLock" false)
    (Variables|/Script/Engine.PlayerController|SetbShowMouseCursor (Game|GetPlayerController 0) true)))

(fn ConstructionScript
  (|CallParentFunction))