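; BP_MoveIntoPlayer is a short-lived jumpscare actor whose skeletal mesh rushes forward, by its name into the player, as a scare sound plays.
; BeginPlay spawns the sound at a hard-coded world location with an attenuation asset, then destroys the actor after a one-second delay.
; Tick slides the mesh toward the Arrow component's position at constant speed using VInterpToConstant, without sweeping for collision.
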(event EventBeginPlay
  (|CallParentFunction)
  (Audio|SpawnSoundatLocation "/Game/_Main/Sounds/SFX/SFX_Jumpscare_1.SFX_Jumpscare_1" "-1012.000008,-1008.509200,238.292512" "0, 0, 0" 1.0 1.0 0.0 "/Game/_Main/Sounds/SA_LittleGirlCry.SA_LittleGirlCry" 0)
  (Utilities|FlowControl|Delay 1.0)
  (Actor|DestroyActor))

(event EventTick
  (params (DeltaSeconds :type Float%20%28single-precision%29))
  (Transformation|SetWorldLocation (Variables|Default|GetSkeletalMesh) (Math|Interpolation|VInterptoConstant (Transformation|GetWorldLocation (Variables|Default|GetSkeletalMesh)) (Transformation|GetWorldLocation (Variables|Default|GetArrow)) DeltaSeconds 1e+03) false false))

(fn ConstructionScript
  (|CallParentFunction))