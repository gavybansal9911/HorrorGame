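; Little girl jumpscare actor meant to jump on the player once she sees them, though TriggerScare currently only prints a debug string.
; On BeginPlay it plays a low-pitched scream at EyesLocation, then destroys itself after a 30-second delay.
; Until scared, Tick sphere-traces on Visibility from the eyes, firing TriggerScare once on a Player-tagged hit.
; The trace end multiplies eye location by the scaled forward vector instead of adding it.
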(event Custom|Trigger%20Scare
  (Development|PrintString "Jump On Player!"))

(event EventBeginPlay
  (Audio|SpawnSoundatLocation "/Game/_Main/Sounds/Girl/Girl_screaming_1.Girl_screaming_1" (Transformation|GetWorldLocation (Variables|Default|GetEyesLocation)) "0, 0, 0" 1.3 0.4 0.0 "/Game/_Main/Sounds/SA_LittleGirlScream.SA_LittleGirlScream" 0)
  (Utilities|FlowControl|Delay 3e+01)
  (Actor|DestroyActor))

(event EventTick
  (params (DeltaSeconds :type Float%20%28single-precision%29))
  (bind _eyeslocation (Variables|Default|GetEyesLocation))
  (bind _returnvalue (Transformation|GetWorldLocation _eyeslocation))
  (if (not (Variables|Default|GetbScared))
    (bind (_outhit _returnvalue_2) (Collision|SphereTraceByChannel _returnvalue (* _returnvalue (* (Transformation|GetActorForwardVector) 1e+05)) 5e+01 "TraceTypeQuery1" false (Utilities|Array|MakeArray self) "None"))
    (if _returnvalue_2
      (if (Actor|ActorHasTag (.HitActor (Collision|BreakHitResult _outhit)) "Player")
        (Variables|Default|SetbScared true)
        (CallFunction|TriggerScare)))))

(fn ConstructionScript
  (|CallParentFunction))