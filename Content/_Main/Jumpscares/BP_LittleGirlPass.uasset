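; BP_LittleGirlPass is a brief jumpscare actor in which a skeletal mesh, by its name a little girl, rushes past.
; On spawn it plays a jumpscare sound with little-girl-cry attenuation at a hardcoded world location, then destroys itself after a one-second delay.
; Every tick it slides the mesh toward its Arrow component at constant speed using VInterpToConstant, so the arrow marks the end of the pass.
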(event EventBeginPlay
  (|CallParentFunction)
  (Audio|SpawnSoundatLocation "/Game/_Main/Sounds/SFX/SFX_Jumpscare_1.SFX_Jumpscare_1" "1886.990234,-669.759583,599.999939" "0, 0, 0" 12.5 1.0 7.0 "/Game/_Main/Sounds/SA_LittleGirlCry.SA_LittleGirlCry" 0)
  (Utilities|FlowControl|Delay 1.0)
  (Actor|DestroyActor))

(event EventTick
  (params (DeltaSeconds :type Float%20%28single-precision%29))
  (Transformation|SetWorldLocation (Variables|Default|GetSkeletalMesh) (Math|Interpolation|VInterptoConstant (Transformation|GetWorldLocation (Variables|Default|GetSkeletalMesh)) (Transformation|GetWorldLocation (Variables|Default|GetArrow)) DeltaSeconds 7e+02) false false))

(fn ConstructionScript
  (|CallParentFunction))