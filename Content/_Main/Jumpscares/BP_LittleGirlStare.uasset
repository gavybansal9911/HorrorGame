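; BP_LittleGirlStare is a jumpscare actor: a ghostly girl who stares at the player and vanishes when approached.
; On BeginPlay it sequences idle, take-off and looping hover animations using timed delays.
; Tick turns the mesh's yaw toward the first-person camera, with a 90-degree offset.
; Player overlap with the Box triggers a single VInterpTo step toward their XY, with Current unset, then destroys the actor after a short delay.
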(event OnComponentBeginOverlap(Box)
  (params (OverlappedComponent :type Primitive%20Component%20Object%20Reference) (OtherActor :type Actor%20Object%20Reference) (OtherComp :type Primitive%20Component%20Object%20Reference) (OtherBodyIndex :type Integer) (bFromSweep :type Boolean) (SweepResult :type Hit%20Result%20Structure%20%28by%20ref%29))
  (bind _asbp_first_person_character (Utilities|Casting|CastToBP_FirstPersonCharacter OtherActor))
  (Development|PrintString "Haunt Player Now!")
  (Transformation|SetWorldLocation (Variables|Default|GetSkeletalMesh) (Math|Interpolation|VInterpTo "0, 0, 0" (Math|Vector|MakeVector (.x (Transformation|GetActorLocation _asbp_first_person_character)) (.y (Transformation|GetActorLocation _asbp_first_person_character)) (.z (Transformation|GetWorldLocation (Variables|Default|GetSkeletalMesh)))) (Utilities|Time|GetWorldDeltaSeconds) 1e+02) false false)
  (Utilities|FlowControl|Delay 0.5)
  (Actor|DestroyActor))

(event EventBeginPlay
  (Components|Animation|PlayAnimation (Variables|Default|GetSkeletalMesh) "/Game/HorrorGirl/Animation/HorrorGirl_root_Idel.HorrorGirl_root_Idel" true)
  (Utilities|FlowControl|Delay 3.0)
  (Components|Animation|PlayAnimation (Variables|Default|GetSkeletalMesh) "/Game/HorrorGirl/Animation/HorrorGirl_root_StartFly.HorrorGirl_root_StartFly" false)
  (Utilities|FlowControl|Delay 2.0)
  (Components|Animation|PlayAnimation (Variables|Default|GetSkeletalMesh) "/Game/HorrorGirl/Animation/HorrorGirl_root_Fly_Idel.HorrorGirl_root_Fly_Idel" true))

(event EventTick
  (params (DeltaSeconds :type Float%20%28single-precision%29))
  (bind _asbp_first_person_character (Utilities|Casting|CastToBP_FirstPersonCharacter (Game|GetPlayerCharacter 0)))
  (Transformation|SetWorldRotation (Variables|Default|GetSkeletalMesh) (Math|Rotator|MakeRotator 0.0 0.0 (- (.yaw (Math|Rotator|FindLookatRotation (Transformation|GetWorldLocation (Variables|Default|GetSkeletalMesh)) (Transformation|GetWorldLocation (Variables|/Game/FirstPerson/Blueprints/BP_FirstPersonCharacter.BP_FirstPersonCharacter_C|GetFirstPersonCamera _asbp_first_person_character)))) 9e+01)) false false))

(fn ConstructionScript
  (|CallParentFunction))