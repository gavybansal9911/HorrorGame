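; Box trigger volume that fires configured horror events when the first-person player overlaps it.
; Begin overlap, and optionally end overlap, feeds the event list to the CheckEvent macro, with options for one-shot triggering and self-destruction on exit.
; CheckEvent dispatches environment actions by type (lock, interact, switch off, delayed spawn, light flicker), then messages player and sound targets through I_InteractInterface.
; Interact actions can repeat on a delay while the player stays inside.
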(event OnComponentBeginOverlap(Box)
  (params (OverlappedComponent :type Primitive%20Component%20Object%20Reference) (OtherActor :type Actor%20Object%20Reference) (OtherComp :type Primitive%20Component%20Object%20Reference) (OtherBodyIndex :type Integer) (bFromSweep :type Boolean) (SweepResult :type Hit%20Result%20Structure%20%28by%20ref%29))
  (bind _asbp_first_person_character (Utilities|Casting|CastToBP_FirstPersonCharacter OtherActor))
  (if (not (Variables|Bools|GetbOverlapOnce))
    (Development|PrintString "Overlap Triggered")
    (Variables|Bools|SetPlayer%20Overlapped true)
    (Utilities|CheckEvent (Variables|HorrorEvent|GetHorror%20Events) _asbp_first_person_character (Variables|/Game/FirstPerson/Blueprints/BP_FirstPersonCharacter.BP_FirstPersonCharacter_C|GetGrabbed%20Object _asbp_first_person_character)
      (:Completed
        (if (not (Variables|Bools|GetbCanOverlapAgain))
          (Variables|Bools|SetbOverlapOnce true))))))

(event OnComponentEndOverlap(Box)
  (params (OverlappedComponent :type Primitive%20Component%20Object%20Reference) (OtherActor :type Actor%20Object%20Reference) (OtherComp :type Primitive%20Component%20Object%20Reference) (OtherBodyIndex :type Integer))
  (bind _asbp_first_person_character (Utilities|Casting|CastToBP_FirstPersonCharacter OtherActor))
  (Utilities|FlowControl|Sequence
    (:then_0
      (Development|PrintString "Overlap Trigger End")
      (Variables|Bools|SetPlayer%20Overlapped false)
      (if (Variables|Bools|GetbTriggerEventOnEndOverlap)
        (Utilities|CheckEvent (Variables|HorrorEvent|GetHorror%20Events) _asbp_first_person_character (Variables|/Game/FirstPerson/Blueprints/BP_FirstPersonCharacter.BP_FirstPersonCharacter_C|GetGrabbed%20Object _asbp_first_person_character))))
    (:then_1
      (if (Variables|Default|GetbDestoryOnEndOverlap)
        (Actor|DestroyActor)))))

(fn ConstructionScript)