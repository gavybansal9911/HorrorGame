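; AI controller for the monk enemy, running BT_AI_Monk and feeding its blackboard from perception and player state.
; Seeing a non-hiding player sets sight and pursuit flags, while losing perception clears sight and re-arms the jumpscare audio flag.
; Heard noises set a sound flag and store the stimulus location as the target.
; The player character's hide event mirrors its hiding state into the blackboard.
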(event OnTargetPerceptionUpdated(AIPerception)
  (params (Actor :type Actor%20Object%20Reference) (Stimulus :type AI%20Stimulus%20Structure))
  (CallFunction|HandleSoundSense Stimulus)
  (bind _asbp_first_person_character (Utilities|Casting|CastToBP_FirstPersonCharacter Actor))
  (if (.bSuccessfullySensed (Utilities|Struct|BreakAIStimulus Stimulus))
    (if (not (Variables|/Game/FirstPerson/Blueprints/BP_FirstPersonCharacter.BP_FirstPersonCharacter_C|GetIsHiding? _asbp_first_person_character))
      (AI|Components|Blackboard|SetValueasBool (AI|GetBlackboard self) (Utilities|Name|MakeLiteralName "CanSeePlayer") true)
      (AI|Components|Blackboard|SetValueasBool (AI|GetBlackboard self) (Utilities|Name|MakeLiteralName "IsPursuingPlayer") true))
    (else
      (AI|Components|Blackboard|SetValueasBool (AI|GetBlackboard self) (Utilities|Name|MakeLiteralName "CanSeePlayer") false)
      (AI|Components|Blackboard|SetValueasBool (AI|GetBlackboard 0) (Utilities|Name|MakeLiteralName "PlayJumpscareAudio") true))))

(event Custom|Set%20IsPlayerHidden
  (bind _output_get (Variables|Default|SetbIsPlayerHiding (Variables|/Game/FirstPerson/Blueprints/BP_FirstPersonCharacter.BP_FirstPersonCharacter_C|GetIsHiding? (stale EventBeginPlay _asbp_first_person_character))))
  (AI|Components|Blackboard|SetValueasBool (AI|GetBlackboard 0) (Utilities|Name|MakeLiteralName "IsPlayerHidden") _output_get)
  (Development|PrintString (Utilities|String|ToString(Boolean) _output_get)))

(event EventBeginPlay
  (AI|RunBehaviorTree "/Game/_Main/AI/BT_AI_Monk.BT_AI_Monk")
  (AI|Components|Blackboard|SetValueasBool (AI|GetBlackboard 0) (Utilities|Name|MakeLiteralName "PlayJumpscareAudio") true)
  (Utilities|FlowControl|Delay 0.1)
  (bind _asbp_first_person_character (Utilities|Casting|CastToBP_FirstPersonCharacter (Game|GetPlayerCharacter 0)))
  (EventDispatchers|BindEventtoOnPlayerHide _asbp_first_person_character (delegate Custom|Set%20IsPlayerHidden)))

(fn ConstructionScript)

(fn HandleSoundSense
  (params (Stimulas :type AI%20Stimulus%20Structure))
  (bind _returnvalue (Class|AIPerceptionSystem|GetSenseClassforStimulus Stimulas))
  (if (== _returnvalue "/Script/AIModule.AISense_Hearing")
    (AI|Components|Blackboard|SetValueasBool (AI|GetBlackboard self) (Utilities|Name|MakeLiteralName "SoundHeared") true)
    (AI|Components|Blackboard|SetValueasVector (AI|GetBlackboard self) (Utilities|Name|MakeLiteralName "TargetLocation") (.StimulusLocation (Utilities|Struct|BreakAIStimulus Stimulas)))))